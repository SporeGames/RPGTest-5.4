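; BP_ObjKillEnemie is a quest objective that completes when a designated enemy actor is destroyed.
; On activation it runs the parent objective logic and binds to the target's OnDestroyed event.
; When that fires, it unbinds, prints a debug string, sets a Dead flag and broadcasts OnCompleted, while GetIsComplete reports that flag.
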(event `self.ActivateObjective`
  (`parent.ActivateObjective`)
  (add `Actor.OnDestroyed` (`self.EnemieToDie`) (delegate `OnDeath`)))

(event `OnDeath`
  (params (DestroyedActor :type "Actor Object Reference"))
  (remove `Actor.OnDestroyed` (`self.EnemieToDie`) (delegate `OnDeath`))
  (`KismetSystemLibrary.PrintString` null "Dead")
  (set `self.Dead` true)
  (`self.OnCompleted` self))

(fn `GetIsComplete`
  (returns (IsComplete :type Boolean))
  (return (`self.Dead`)))