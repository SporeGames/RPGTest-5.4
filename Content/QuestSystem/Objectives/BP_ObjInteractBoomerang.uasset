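; Quest objective Blueprint that completes when the player interacts with a boomerang.
; On activation it calls the parent logic and binds to the boomerang's CallQuest dispatcher.
; When that fires, it unbinds, sets an Interacted flag and broadcasts OnCompleted, and GetIsComplete returns that flag.
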(event `self.ActivateObjective`
  (`parent.ActivateObjective`)
  (add `/Game/Blueprints/Interactables/BP_Item_Boomerang.CallQuest` (`self.Boomerang`) (delegate `InteractedEvent`)))

(event `InteractedEvent`
  (remove `/Game/Blueprints/Interactables/BP_Item_Boomerang.CallQuest` (`self.Boomerang`) (delegate `InteractedEvent`))
  (set `self.Interacted` true)
  (`self.OnCompleted` self))

(fn `GetIsComplete`
  (returns (IsComplete :type Boolean))
  (return (`self.Interacted`)))