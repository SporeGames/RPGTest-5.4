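; BP_ObjKillXEnemies is a quest objective for killing a set list of enemies.
; Death_Event removes the killed enemy from EnemiesToKill, increments KillCounter, and completes the objective when the list empties.
; Its name shows the count against a hard-coded total of 4.
; Death binding nodes are disconnected, so the activation loop does nothing and this graph never binds Death_Event.
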(event `self.ActivateObjective`
  (`parent.ActivateObjective`)
  (set `self.Length` (`KismetArrayLibrary.Array_Length` (`self.EnemiesToKill`)))
  (for _array_element (`self.EnemiesToKill`)
    _))

(event `Death_Event`
  (params (KilledEnemy :type "/Game/Blueprints/Enemies/BP_Enemy_Parent Object Reference"))
  (`KismetArrayLibrary.Array_RemoveItem` (`self.EnemiesToKill`) KilledEnemy)
  (bind _result (`/Engine/EditorBlueprintResources/StandardMacros.IncrementInt` (`self.KillCounter`))
    (:`  `
      (set `self.KillCounter` _result)
      (if (<= (`KismetArrayLibrary.Array_Length` (`self.EnemiesToKill`)) 0)
        (set `self.AllDead` true)
        (`self.OnCompleted` self)))))

(fn `GetIsComplete`
  (returns (IsComplete :type Boolean))
  (return (`self.AllDead`)))

(fn `GetObjectiveName`
  (returns (ObjectiveName :type Text))
  (return (`|FormatText` "Kill Enemies {index}/4{m}" (`self.KillCounter`) _)))