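; BP_Objective is a quest system objective that exposes a name, image, active state and completion state.
; ActivateObjective sets the active flag, and simple getters return the name, image and flag.
; GetIsComplete always returns true, with no condition checked.
; IncreaseDialogNPC is empty as wired: its nodes for advancing a linked NPC's dialog tree counter are disconnected and never run.
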(event `ActivateObjective`
  (set `self.IsActive` true))

(fn `GetIsActive`
  (returns (IsAcive :type Boolean))
  (return (`self.IsActive`)))

(fn `GetIsComplete`
  (returns (IsComplete :type Boolean))
  (return true))

(fn `GetObjectiveImage`
  (returns (Image :type "Texture2D Object Reference"))
  (return (`self.Image`)))

(fn `GetObjectiveName`
  (returns (ObjectiveName :type Text))
  (return (`self.ObjectiveName`)))

(fn `IncreaseDialogNPC`)