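; BP_ObjCollectItem is a quest objective that completes when the player interacts with its referenced item.
; On activation it runs the parent logic and binds to the item's OnInteracted event.
; The interaction handler unbinds itself, sets the Collected flag and broadcasts OnCompleted, while GetIsComplete reports that flag.
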(event `self.ActivateObjective`
  (`parent.ActivateObjective`)
  (add `/Game/Blueprints/Interactables/BP_Item_Parent.OnInteracted` (`self.Item`) (delegate `ItemCollected`)))

(event `ItemCollected`
  (remove `/Game/Blueprints/Interactables/BP_Item_Parent.OnInteracted` (`self.Item`) (delegate `ItemCollected`))
  (set `self.Collected` true)
  (`self.OnCompleted` self))

(fn `GetIsComplete`
  (returns (IsComplete :type Boolean))
  (return (`self.Collected`)))