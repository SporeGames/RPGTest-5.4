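; BP_ObjInteractWithCheckpoint is a quest objective that completes when its InteractableCheckpoint is interacted with.
; On activation it runs the parent logic, prints a debug string and binds InteractedWithNPC to the checkpoint through BindEventToQuest.
; When that event fires, it unbinds itself, sets the Interacted flag and calls OnCompleted with itself.
; GetIsComplete returns the Interacted flag.
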(event `self.ActivateObjective`
  (`parent.ActivateObjective`)
  (`KismetSystemLibrary.PrintString` null "ACTIVE")
  (add `/Game/Blueprints/Interactables/BP_Checkpoint.Quest` (`self.InteractableCheckpoint`) (delegate `InteractedWithNPC`)))

(event `InteractedWithNPC`
  (remove `/Game/Blueprints/Interactables/BP_Checkpoint.OnInteracted` (`self.InteractableCheckpoint`) (delegate `InteractedWithNPC`))
  (set `self.Interacted` true)
  (`self.OnCompleted` self))

(fn `GetIsComplete`
  (returns (IsComplete :type Boolean))
  (return (`self.Interacted`)))