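; BP_ObjHitTarget is a quest objective that completes when a designated enemy is hit.
; On activation it calls the parent and binds to the OnHit event of EnemieToHit.
; The first hit unbinds the listener, sets a Hit flag that GetIsComplete returns, and fires the OnCompleted dispatcher with itself.
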(event `self.ActivateObjective`
  (`parent.ActivateObjective`)
  (add `/Game/Blueprints/BP_Dummy.OnHit` (`self.Enemie To Hit`) (delegate `OnHit`)))

(event `OnHit`
  (remove `/Game/Blueprints/BP_Dummy.OnHit` (`self.Enemie To Hit`) (delegate `OnHit`))
  (set `self.Hit` true)
  (`self.OnCompleted` self))

(fn `GetIsComplete`
  (returns (IsComplete :type Boolean))
  (return (`self.Hit`)))