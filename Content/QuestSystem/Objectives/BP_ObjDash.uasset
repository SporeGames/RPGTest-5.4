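; BP_ObjDash is a quest objective that completes when the player unlocks the dash ability.
; On activation it binds to the CallQuest event reached through the checkpoint skill tree.
; When that fires, it prints a debug message, unbinds itself, sets the Unlocked flag and broadcasts completion.
; GetIsComplete returns that flag.
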(event `self.ActivateObjective`
  (`parent.ActivateObjective`)
  (add `/Game/UI/WB_Skilltree.CallQuest` (`/Game/Blueprints/Interactables/BP_Checkpoint.NewVar` (`self.CheckpointSkillTree`)) (delegate `UnlockedDash`)))

(event `UnlockedDash`
  (`KismetSystemLibrary.PrintString` null "DASH Unlocked" true true (struct :`R` 0.114583 :`G` 0.008027 :`B` 0.081492 :`A` 1.0) 10.0)
  (remove `/Game/UI/WB_Skilltree.CallQuest` (`/Game/Blueprints/Interactables/BP_Checkpoint.NewVar` (`self.CheckpointSkillTree`)) (delegate `UnlockedDash`))
  (set `self.Unlocked` true)
  (`self.OnCompleted` self))

(fn `GetIsComplete`
  (returns (IsComplete :type Boolean))
  (return (`self.Unlocked`)))