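; BP_Quest_Tutorialoptb is a tutorial quest with German objective text about saying goodbye, talking to Mum and training on straw dummies.
; It overrides the parent quest's construction hooks to build an order-required root objective collection.
; It fills that collection with three objectives: an NPC interaction with Mum, a hit-target objective tied to NPC1, and a second talk with Mum.
; The event graph holds only disabled stubs.
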(fn `ConstructRootObjectiveCollection`
  (returns (RootObjCollection :type "/Game/QuestSystem/Objectives/BP_ObjCollection Object Reference"))
  (bind _returnvalue (`|GenericCreateObject` "/Game/QuestSystem/Objectives/BP_ObjCollection.BP_ObjCollection_C" true "2Verabschiede dich." true 0 "" (`self.Image`)))
  (return _returnvalue))

(fn `PopulateObjectives`
  (params (RootObjCollection :type "/Game/QuestSystem/Objectives/BP_ObjCollection Object Reference") (`NPC 1` :type "/Game/Blueprints/NPC/BP_NPC Object Reference") (`NPC 2` :type "/Game/Blueprints/NPC/BP_NPC Object Reference"))
  (`|ExecutionSequence`
    (:`then_0`
      (bind _returnvalue (`|GenericCreateObject` "/Game/QuestSystem/Objectives/BP_InteractWithNPC.BP_InteractWithNPC_C" (`self.Mum`) "Rede mit Mama" false 0 "" null))
      (`/Game/QuestSystem/Objectives/BP_ObjCollection.AddObjective` (`local.RootObjCollection`) _returnvalue null self))
    (:`then_1`
      (bind _returnvalue_2 (`|GenericCreateObject` "/Game/QuestSystem/Objectives/BP_ObjHitTarget.BP_ObjHitTarget_C" (`self.Bommerang`) "Trainiere mit den Strohpuppen" false 0 "" null))
      (`/Game/QuestSystem/Objectives/BP_ObjCollection.AddObjective` (`local.RootObjCollection`) _returnvalue_2 `NPC 1` self))
    (:`then_2`
      (bind _returnvalue_3 (`|GenericCreateObject` "/Game/QuestSystem/Objectives/BP_InteractWithNPC.BP_InteractWithNPC_C" (`self.Mum 2`) "Rede nochmal mit Mama" false 0 "" null))
      (`/Game/QuestSystem/Objectives/BP_ObjCollection.AddObjective` (`local.RootObjCollection`) _returnvalue_3 null self))))

(fn `UserConstructionScript`
  (`parent.UserConstructionScript`))