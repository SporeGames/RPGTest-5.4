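; BP_Quest_1 is a combat quest that tracks hitting a set of training dummies.
; It builds a root objective collection named "Combat" with an image.
; It then adds one hit-target objective per entry in DummysToHit, each labeled with its numbered position.
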(fn `ConstructRootObjectiveCollection`
  (returns (RootObjCollection :type "/Game/QuestSystem/Objectives/BP_ObjCollection Object Reference"))
  (bind _returnvalue (`|GenericCreateObject` "/Game/QuestSystem/Objectives/BP_ObjCollection.BP_ObjCollection_C" false "Combat" true 0 "" (`self.Image`)))
  (return _returnvalue))

(fn `PopulateObjectives`
  (params (RootObjCollection :type "/Game/QuestSystem/Objectives/BP_ObjCollection Object Reference") (`NPC 1` :type "/Game/Blueprints/NPC/BP_NPC Object Reference") (`NPC 2` :type "/Game/Blueprints/NPC/BP_NPC Object Reference"))
  (for (_array_element _array_index) (`self.DummysToHit`)
    (bind _returnvalue (`|GenericCreateObject` "/Game/QuestSystem/Objectives/BP_ObjHitTarget.BP_ObjHitTarget_C" _array_element (`|FormatText` "Hit Dummy {index}" (+ _array_index 1)) false 0 "" null))
    (`/Game/QuestSystem/Objectives/BP_ObjCollection.AddObjective` (`local.RootObjCollection`) _returnvalue null null)))

(fn `UserConstructionScript`
  (`parent.UserConstructionScript`))