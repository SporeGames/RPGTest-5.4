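; BP_Quest_NQ2 is a level 4 quest where the player helps Gangolf at a memorial by placing keepsakes for the dead, then saying goodbye.
; It builds an unordered root objective collection, so order is not required.
; PopulateObjectives adds three place-item objectives at named graves, the third also passed NPC1, plus an NPC-interaction farewell.
; The event graph holds no active logic.
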(fn `ConstructRootObjectiveCollection`
  (returns (RootObjCollection :type "/Game/QuestSystem/Objectives/BP_ObjCollection Object Reference"))
  (bind _returnvalue (`|GenericCreateObject` "/Game/QuestSystem/Objectives/BP_ObjCollection.BP_ObjCollection_C" false "Helfe Gangolf bei der Gedenkstätte."))
  (return _returnvalue))

(fn `PopulateObjectives`
  (params (RootObjCollection :type "/Game/QuestSystem/Objectives/BP_ObjCollection Object Reference") (`NPC 1` :type "/Game/Blueprints/NPC/BP_NPC Object Reference") (`NPC 2` :type "/Game/Blueprints/NPC/BP_NPC Object Reference"))
  (`|ExecutionSequence`
    (:`then_0`
      (bind _returnvalue (`|GenericCreateObject` "/Game/QuestSystem/Objectives/BP_ObjPlaceItem.BP_ObjPlaceItem_C" (`self.Claire´s Grab`) "Lege den Teddy zu Claire´s \"Grab\"."))
      (`/Game/QuestSystem/Objectives/BP_ObjCollection.AddObjective` (`local.RootObjCollection`) _returnvalue null self))
    (:`then_1`
      (bind _returnvalue_2 (`|GenericCreateObject` "/Game/QuestSystem/Objectives/BP_ObjPlaceItem.BP_ObjPlaceItem_C" (`self.Fraus Grab`) "Lege das Gemälde für die Frau hin."))
      (`/Game/QuestSystem/Objectives/BP_ObjCollection.AddObjective` (`local.RootObjCollection`) _returnvalue_2 null self))
    (:`then_2`
      (bind _returnvalue_3 (`|GenericCreateObject` "/Game/QuestSystem/Objectives/BP_ObjPlaceItem.BP_ObjPlaceItem_C" (`self.Bruder´s Grab`) "Hole die Blume für den Bruder."))
      (`/Game/QuestSystem/Objectives/BP_ObjCollection.AddObjective` (`local.RootObjCollection`) _returnvalue_3 `NPC 1` self))
    (:`then_3`
      (bind _returnvalue_4 (`|GenericCreateObject` "/Game/QuestSystem/Objectives/BP_InteractWithNPC.BP_InteractWithNPC_C" null "Verabschiede dich von Gangolf"))
      (`/Game/QuestSystem/Objectives/BP_ObjCollection.AddObjective` (`local.RootObjCollection`) _returnvalue_4 null self))))

(fn `UserConstructionScript`
  (`parent.UserConstructionScript`))