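; BP_Quest_NQ1 is a Level 4 quest in which the player searches for clues to find out what happened, with objective text in German.
; It builds a root objective collection, then adds three reach-destination objectives, each targeting its own clue reference (Hinweis1 to Hinweis3).
; The NPC inputs to PopulateObjectives go unused, and the event graph and construction script add no logic of their own.
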(fn `ConstructRootObjectiveCollection`
  (returns (RootObjCollection :type "/Game/QuestSystem/Objectives/BP_ObjCollection Object Reference"))
  (bind _returnvalue (`|GenericCreateObject` "/Game/QuestSystem/Objectives/BP_ObjCollection.BP_ObjCollection_C" false "Finde heraus was passiert ist."))
  (return _returnvalue))

(fn `PopulateObjectives`
  (params (RootObjCollection :type "/Game/QuestSystem/Objectives/BP_ObjCollection Object Reference") (`NPC 1` :type "/Game/Blueprints/NPC/BP_NPC Object Reference") (`NPC 2` :type "/Game/Blueprints/NPC/BP_NPC Object Reference"))
  (`|ExecutionSequence`
    (:`then_0`
      (bind _returnvalue (`|GenericCreateObject` "/Game/QuestSystem/Objectives/BP_ObjRechDestination.BP_ObjRechDestination_C" (`self.Hinweis 1`) "Suche nach Hinweisen 1."))
      (`/Game/QuestSystem/Objectives/BP_ObjCollection.AddObjective` (`local.RootObjCollection`) _returnvalue null self))
    (:`then_1`
      (bind _returnvalue_2 (`|GenericCreateObject` "/Game/QuestSystem/Objectives/BP_ObjRechDestination.BP_ObjRechDestination_C" (`self.Hinweis 2`) "Suche nach Hinweisen 2."))
      (`/Game/QuestSystem/Objectives/BP_ObjCollection.AddObjective` (`local.RootObjCollection`) _returnvalue_2 null self))
    (:`then_2`
      (bind _returnvalue_3 (`|GenericCreateObject` "/Game/QuestSystem/Objectives/BP_ObjRechDestination.BP_ObjRechDestination_C" (`self.Hinweis 3`) "Suche nach Hinweisen 3."))
      (`/Game/QuestSystem/Objectives/BP_ObjCollection.AddObjective` (`local.RootObjCollection`) _returnvalue_3 null self))))

(fn `UserConstructionScript`
  (`parent.UserConstructionScript`))