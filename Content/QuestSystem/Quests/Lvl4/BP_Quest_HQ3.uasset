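; BP_Quest_HQ3 is a Lvl4 quest that defines an ordered objective chain around finding and releasing Claire.
; It builds an order-required root objective collection, then fills it with reaching the ruin, killing Claire, handing Gangolf the teddy and leaving the island.
; Each step reuses a generic objective class with German display text; the final reach-destination objective receives no destination here.
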(fn `ConstructRootObjectiveCollection`
  (returns (RootObjCollection :type "/Game/QuestSystem/Objectives/BP_ObjCollection Object Reference"))
  (bind _returnvalue (`|GenericCreateObject` "/Game/QuestSystem/Objectives/BP_ObjCollection.BP_ObjCollection_C" true "Finde Claire."))
  (return _returnvalue))

(fn `PopulateObjectives`
  (params (RootObjCollection :type "/Game/QuestSystem/Objectives/BP_ObjCollection Object Reference") (NPC :type "/Game/Blueprints/NPC/BP_NPC Object Reference"))
  (`|ExecutionSequence`
    (:`then_0`
      (bind _returnvalue (`|GenericCreateObject` "/Game/QuestSystem/Objectives/BP_ObjRechDestination.BP_ObjRechDestination_C" (`self.Ruine`) "Finde Claire."))
      (`/Game/QuestSystem/Objectives/BP_ObjCollection.AddObjective` (`local.RootObjCollection`) _returnvalue null self))
    (:`then_1`
      (bind _returnvalue_2 (`|GenericCreateObject` "/Game/QuestSystem/Objectives/BP_ObjKillEnemie.BP_ObjKillEnemie_C" (`self.Claire`) "Erlöse Claire."))
      (`/Game/QuestSystem/Objectives/BP_ObjCollection.AddObjective` (`local.RootObjCollection`) _returnvalue_2 null self))
    (:`then_2`
      (bind _returnvalue_3 (`|GenericCreateObject` "/Game/QuestSystem/Objectives/BP_InteractWithNPC.BP_InteractWithNPC_C" (`self.Gangolf`) "Übergib Gangolf den Teddy."))
      (`/Game/QuestSystem/Objectives/BP_ObjCollection.AddObjective` (`local.RootObjCollection`) _returnvalue_3 null self))
    (:`then_3`
      (bind _returnvalue_4 (`|GenericCreateObject` "/Game/QuestSystem/Objectives/BP_ObjRechDestination.BP_ObjRechDestination_C" null "Verlasse die Insel"))
      (`/Game/QuestSystem/Objectives/BP_ObjCollection.AddObjective` (`local.RootObjCollection`) _returnvalue_4 null self))))

(fn `UserConstructionScript`
  (`parent.UserConstructionScript`))