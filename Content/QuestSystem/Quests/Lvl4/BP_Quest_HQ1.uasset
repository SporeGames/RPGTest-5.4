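; BP_Quest_HQ1 is a Level 4 quest that tasks the player with exploring the village ("Erkunde das Dorf.").
; It constructs an unordered root objective collection, then adds a single reach-destination objective targeting SichtungHerzloser and registers it with this quest.
; The NPC inputs go unused, and the event graph and construction script add no logic of their own.
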(fn `ConstructRootObjectiveCollection`
  (returns (RootObjCollection :type "/Game/QuestSystem/Objectives/BP_ObjCollection Object Reference"))
  (bind _returnvalue (`|GenericCreateObject` "/Game/QuestSystem/Objectives/BP_ObjCollection.BP_ObjCollection_C" false "Erkunde das Dorf."))
  (return _returnvalue))

(fn `PopulateObjectives`
  (params (RootObjCollection :type "/Game/QuestSystem/Objectives/BP_ObjCollection Object Reference") (`NPC 1` :type "/Game/Blueprints/NPC/BP_NPC Object Reference") (`NPC 2` :type "/Game/Blueprints/NPC/BP_NPC Object Reference"))
  (`|ExecutionSequence`
    (:`then_0`
      (bind _returnvalue (`|GenericCreateObject` "/Game/QuestSystem/Objectives/BP_ObjRechDestination.BP_ObjRechDestination_C" (`self.Sichtung Herzloser`) "Erkunde das Dorf."))
      (`/Game/QuestSystem/Objectives/BP_ObjCollection.AddObjective` (`local.RootObjCollection`) _returnvalue null self))))

(fn `UserConstructionScript`
  (`parent.UserConstructionScript`))