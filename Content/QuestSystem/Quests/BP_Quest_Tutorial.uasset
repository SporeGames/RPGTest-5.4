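; Tutorial quest that prepares the player for the journey through talking to Mum, hitting dummies and collecting the boomerang.
; It builds an order-required root objective collection, then adds five objectives in sequence: talk to Mum, hit a dummy, pick up the boomerang, hit all dummies with one throw, and talk to Mum again.
; Each step is a constructed objective object for NPC interaction, target hit or destination reached, with German display names.
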(fn `ConstructRootObjectiveCollection`
  (returns (RootObjCollection :type "/Game/QuestSystem/Objectives/BP_ObjCollection Object Reference"))
  (bind _returnvalue (`|GenericCreateObject` "/Game/QuestSystem/Objectives/BP_ObjCollection.BP_ObjCollection_C" true "Bereite dich auf die Reise vor!"))
  (return _returnvalue))

(fn `PopulateObjectives`
  (params (RootObjCollection :type "/Game/QuestSystem/Objectives/BP_ObjCollection Object Reference") (NPC :type "/Game/Blueprints/NPC/BP_NPC Object Reference"))
  (`|ExecutionSequence`
    (:`then_0`
      (bind _returnvalue (`|GenericCreateObject` "/Game/QuestSystem/Objectives/BP_InteractWithNPC.BP_InteractWithNPC_C" (`self.Mum`) "Rede mit Mama."))
      (`/Game/QuestSystem/Objectives/BP_ObjCollection.AddObjective` (`local.RootObjCollection`) _returnvalue null))
    (:`then_1`
      (bind _returnvalue_2 (`|GenericCreateObject` "/Game/QuestSystem/Objectives/BP_ObjHitTarget.BP_ObjHitTarget_C" (`self.Spin Attack`) "Treffe ein Dummy!"))
      (`/Game/QuestSystem/Objectives/BP_ObjCollection.AddObjective` (`local.RootObjCollection`) _returnvalue_2 null))
    (:`then_2`
      (bind _returnvalue_3 (`|GenericCreateObject` "/Game/QuestSystem/Objectives/BP_ObjRechDestination.BP_ObjRechDestination_C" (`self.Boomerang einsammeln`) "Sammel den Bumerang ein."))
      (`/Game/QuestSystem/Objectives/BP_ObjCollection.AddObjective` (`local.RootObjCollection`) _returnvalue_3 null))
    (:`then_3`
      (bind _returnvalue_4 (`|GenericCreateObject` "/Game/QuestSystem/Objectives/BP_ObjHitTarget.BP_ObjHitTarget_C" (`self.Bommerang`) "Treffe alle Dummies mit einem Wurf!"))
      (`/Game/QuestSystem/Objectives/BP_ObjCollection.AddObjective` (`local.RootObjCollection`) _returnvalue_4 NPC))
    (:`then_4`
      (bind _returnvalue_5 (`|GenericCreateObject` "/Game/QuestSystem/Objectives/BP_InteractWithNPC.BP_InteractWithNPC_C" (`self.Mum 2`) "Rede mit Mama."))
      (`/Game/QuestSystem/Objectives/BP_ObjCollection.AddObjective` (`local.RootObjCollection`) _returnvalue_5 null))))

(fn `UserConstructionScript`
  (`parent.UserConstructionScript`))