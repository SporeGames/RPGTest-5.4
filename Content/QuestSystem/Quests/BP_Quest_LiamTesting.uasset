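; Test quest "Respekt den Toten", which has the player find a teddy and bring it to a grave, in that order.
; ConstructRootObjectiveCollection creates the ordered root collection, and PopulateObjectives fills it with collect-item and place-item objectives built from Item and Place.
; A nested objective collection follows as a quest within a quest, holding two placeholder place-item objectives.
; The NPC inputs are unused and the event graph has no active logic.
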(fn `ConstructRootObjectiveCollection`
  (returns (RootObjCollection :type "/Game/QuestSystem/Objectives/BP_ObjCollection Object Reference"))
  (bind _returnvalue (`|GenericCreateObject` "/Game/QuestSystem/Objectives/BP_ObjCollection.BP_ObjCollection_C" true "Respekt den Toten"))
  (return _returnvalue))

(fn `PopulateObjectives`
  (params (RootObjCollection :type "/Game/QuestSystem/Objectives/BP_ObjCollection Object Reference") (`NPC 1` :type "/Game/Blueprints/NPC/BP_NPC Object Reference") (`NPC 2` :type "/Game/Blueprints/NPC/BP_NPC Object Reference"))
  (`|ExecutionSequence`
    (:`then_0`
      ;[1 1 1] NormalQuestStuff
      (bind _returnvalue (`|GenericCreateObject` "/Game/QuestSystem/Objectives/BP_ObjCollectItem.BP_ObjCollectItem_C" (`self.Item`) "Such den Teddy" true 3 "ayo ein teddy"))
      (`/Game/QuestSystem/Objectives/BP_ObjCollection.AddObjective` (`local.RootObjCollection`) _returnvalue null self))
    (:`then_1`
      (bind _returnvalue_2 (`|GenericCreateObject` "/Game/QuestSystem/Objectives/BP_ObjPlaceItem.BP_ObjPlaceItem_C" (`self.Place`) "Bringe den Teddy zum Grab"))
      (`/Game/QuestSystem/Objectives/BP_ObjCollection.AddObjective` (`local.RootObjCollection`) _returnvalue_2 null self))
    (:`then_2`
      ;[0.4479 0.4479 0.4479] Construct Quest in Quest
      (bind _returnvalue_3 (`|GenericCreateObject` "/Game/QuestSystem/Objectives/BP_ObjCollection.BP_ObjCollection_C" false "Quest in Quest" false))
      (bind _output_get (set `self.QuestInQuestRootCollection` _returnvalue_3))
      (`/Game/QuestSystem/Objectives/BP_ObjCollection.AddObjective` (`local.RootObjCollection`) _output_get null self))
    (:`then_3`
      ;[1 1 1] Comment
      (bind _returnvalue_4 (`|GenericCreateObject` "/Game/QuestSystem/Objectives/BP_ObjPlaceItem.BP_ObjPlaceItem_C" (`self.Place`) "Objective"))
      (`/Game/QuestSystem/Objectives/BP_ObjCollection.AddObjective` (`self.QuestInQuestRootCollection`) _returnvalue_4 null self))
    (:`then_4`
      (bind _returnvalue_5 (`|GenericCreateObject` "/Game/QuestSystem/Objectives/BP_ObjPlaceItem.BP_ObjPlaceItem_C" (`self.Place`) "Objective"))
      (`/Game/QuestSystem/Objectives/BP_ObjCollection.AddObjective` (`self.QuestInQuestRootCollection`) _returnvalue_5 null self))))

(fn `UserConstructionScript`
  (`parent.UserConstructionScript`))