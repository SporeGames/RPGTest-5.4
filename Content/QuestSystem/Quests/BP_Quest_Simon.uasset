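; BP_Quest_Simon is a quest Blueprint that tasks the player with greeting the NPC Simon from Römse.
; It creates an unordered root objective collection named "Greet Simon" in ConstructRootObjectiveCollection.
; PopulateObjectives adds a single interact-with-NPC objective to that collection, using the NPC passed into the function.
; The event graph holds only disabled default events, so these two functions define the whole quest.
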(fn `ConstructRootObjectiveCollection`
  (returns (RootObjCollection :type "/Game/QuestSystem/Objectives/BP_ObjCollection Object Reference"))
  (bind _returnvalue (`|GenericCreateObject` "/Game/QuestSystem/Objectives/BP_ObjCollection.BP_ObjCollection_C" false "Greet Simon"))
  (return _returnvalue))

(fn `PopulateObjectives`
  (params (RootObjCollection :type "/Game/QuestSystem/Objectives/BP_ObjCollection Object Reference") (NPC :type "/Game/NPC/BP_NPC Object Reference"))
  (bind _returnvalue (`|GenericCreateObject` "/Game/QuestSystem/Objectives/BP_InteractWithNPC.BP_InteractWithNPC_C" (`self.NPC`) "Greet Simon from Römse"))
  (`/Game/QuestSystem/Objectives/BP_ObjCollection.AddObjective` (`local.RootObjCollection`) _returnvalue null))

(fn `UserConstructionScript`
  (`parent.UserConstructionScript`))