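; BP_Quest is the base quest Blueprint, built around a root objective collection that subclasses are expected to supply and fill.
; On BeginPlay it constructs and stores that collection, populates it using NPCToIncreaseDialog, then activates it.
; ConstructRootObjectiveCollection and PopulateObjectives are template-method stubs that only print errors in the base class.
; A getter exposes the root collection, and the FinishQuest event is empty.
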(event `self.ReceiveBeginPlay`
  (bind _rootobjcollection (`self.ConstructRootObjectiveCollection`))
  (bind _output_get (set `self.RootObjectiveCollection` _rootobjcollection))
  (`self.PopulateObjectives` _output_get (`self.NPCToIncreaseDialog`))
  (`/Game/QuestSystem/Objectives/BP_Objective.ActivateObjective` (`self.RootObjectiveCollection`)))

(event `FinishQuest`)

(fn `ConstructRootObjectiveCollection`
  (returns (RootObjCollection :type "/Game/QuestSystem/Objectives/BP_ObjCollection Object Reference"))
  (`KismetSystemLibrary.PrintString` "Error: CreateRootObjectiveCollection called for base class!" true true (struct :`R` 1.0 :`G` 0.023868 :`A` 1.0))
  (return null))

(fn `GetRootObjectiveCollection`
  (returns (RootObjectiveCollection :type "/Game/QuestSystem/Objectives/BP_ObjCollection Object Reference"))
  (return (`self.RootObjectiveCollection`)))

(fn `PopulateObjectives`
  (params (RootObjCollection :type "/Game/QuestSystem/Objectives/BP_ObjCollection Object Reference") (NPC :type "/Game/NPC/BP_NPC Object Reference"))
  (`KismetSystemLibrary.PrintString` "Error: PopulateObjectives called for base class!" true true (struct :`R` 1.0 :`G` 0.023868 :`A` 1.0)))

(fn `UserConstructionScript`)