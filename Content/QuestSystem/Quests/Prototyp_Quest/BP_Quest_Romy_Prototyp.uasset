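; Prototype quest "Get to know Romy", which has the player talk to Romy, find the forest, kill an enemy and return for a reward.
; ConstructRootObjectiveCollection creates an order-required BP_ObjCollection as the quest root.
; PopulateObjectives adds the four steps as interact, reach-destination and kill objective objects, using NPC, Destination and EnemieToDie as targets.
; The event graph holds only disabled default events.
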(fn `ConstructRootObjectiveCollection`
  (returns (RootObjCollection :type "/Game/QuestSystem/Objectives/BP_ObjCollection Object Reference"))
  (bind _returnvalue (`|GenericCreateObject` "/Game/QuestSystem/Objectives/BP_ObjCollection.BP_ObjCollection_C" true "Get to know Romy"))
  (return _returnvalue))

(fn `PopulateObjectives`
  (params (RootObjCollection :type "/Game/QuestSystem/Objectives/BP_ObjCollection Object Reference") (`NPC 1` :type "/Game/Blueprints/NPC/BP_NPC Object Reference") (`NPC 2` :type "/Game/Blueprints/NPC/BP_NPC Object Reference"))
  (`|ExecutionSequence`
    (:`then_0`
      (bind _returnvalue (`|GenericCreateObject` "/Game/QuestSystem/Objectives/BP_InteractWithNPC.BP_InteractWithNPC_C" (`self.NPC`) "Go find Romy and talk to her"))
      (`/Game/QuestSystem/Objectives/BP_ObjCollection.AddObjective` (`local.RootObjCollection`) _returnvalue null null))
    (:`then_1`
      (bind _returnvalue_2 (`|GenericCreateObject` "/Game/QuestSystem/Objectives/BP_ObjRechDestination.BP_ObjRechDestination_C" (`self.Destination`) "Find the Forest"))
      (`/Game/QuestSystem/Objectives/BP_ObjCollection.AddObjective` (`local.RootObjCollection`) _returnvalue_2 null null))
    (:`then_2`
      (bind _returnvalue_3 (`|GenericCreateObject` "/Game/QuestSystem/Objectives/BP_ObjKillEnemie.BP_ObjKillEnemie_C" (`self.Enemie to Die`) "Kill the enemy"))
      (`/Game/QuestSystem/Objectives/BP_ObjCollection.AddObjective` (`local.RootObjCollection`) _returnvalue_3 null null))
    (:`then_3`
      (bind _returnvalue_4 (`|GenericCreateObject` "/Game/QuestSystem/Objectives/BP_InteractWithNPC.BP_InteractWithNPC_C" (`self.NPC`) "Go back to Romy and claim your reward"))
      (`/Game/QuestSystem/Objectives/BP_ObjCollection.AddObjective` (`local.RootObjCollection`) _returnvalue_4 null null))))

(fn `UserConstructionScript`
  (`parent.UserConstructionScript`))