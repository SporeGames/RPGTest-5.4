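; Test quest Blueprint, named "Sarah Quest", that defines a tutorial-like objective chain with German text covering dialogue, combat, dash unlock and leaving the island by ship.
; ConstructRootObjectiveCollection creates the root objective collection with ordering not required.
; PopulateObjectives adds seven objectives of NPC interaction, target hit, destination and checkpoint types, each bound to a referenced target such as Mum, Bommerang or Flugschiff.
; The event graph holds only disabled placeholder events.
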(fn `ConstructRootObjectiveCollection`
  (returns (RootObjCollection :type "/Game/QuestSystem/Objectives/BP_ObjCollection Object Reference"))
  (bind _returnvalue (`|GenericCreateObject` "/Game/QuestSystem/Objectives/BP_ObjCollection.BP_ObjCollection_C" false "Sarah Quest"))
  (return _returnvalue))

(fn `PopulateObjectives`
  (params (RootObjCollection :type "/Game/QuestSystem/Objectives/BP_ObjCollection Object Reference") (NPC :type "/Game/NPC/BP_NPC Object Reference"))
  (`|ExecutionSequence`
    (:`then_0`
      (bind _returnvalue (`|GenericCreateObject` "/Game/QuestSystem/Objectives/BP_InteractWithNPC.BP_InteractWithNPC_C" (`self.Mum`) "Rede mit Mama."))
      (`/Game/QuestSystem/Objectives/BP_ObjCollection.AddObjective` (`local.RootObjCollection`) _returnvalue null))
    (:`then_1`
      (bind _returnvalue_2 (`|GenericCreateObject` "/Game/QuestSystem/Objectives/BP_ObjHitTarget.BP_ObjHitTarget_C" (`self.Spin Attack`) "Treffe ein Dummy!"))
      (`/Game/QuestSystem/Objectives/BP_ObjCollection.AddObjective` (`local.RootObjCollection`) _returnvalue_2 null))
    (:`then_2`
      (bind _returnvalue_3 (`|GenericCreateObject` "/Game/QuestSystem/Objectives/BP_ObjRechDestination.BP_ObjRechDestination_C" (`self.Boomerang einsammeln`) "Sammel den Boomerang ein."))
      (`/Game/QuestSystem/Objectives/BP_ObjCollection.AddObjective` (`local.RootObjCollection`) _returnvalue_3 null))
    (:`then_3`
      (bind _returnvalue_4 (`|GenericCreateObject` "/Game/QuestSystem/Objectives/BP_ObjHitTarget.BP_ObjHitTarget_C" (`self.Bommerang`) "Treffe alle Dummies mit einem Wurf!"))
      (`/Game/QuestSystem/Objectives/BP_ObjCollection.AddObjective` (`local.RootObjCollection`) _returnvalue_4 null))
    (:`then_4`
      (bind _returnvalue_5 (`|GenericCreateObject` "/Game/QuestSystem/Objectives/BP_InteractWithNPC.BP_InteractWithNPC_C" (`self.Mum 2`) "Rede mit Mama."))
      (`/Game/QuestSystem/Objectives/BP_ObjCollection.AddObjective` (`local.RootObjCollection`) _returnvalue_5 null))
    (:`then_5`
      (bind _returnvalue_6 (`|GenericCreateObject` "/Game/QuestSystem/Objectives/BP_ObjInteractWithCheckpoint.BP_ObjInteractWithCheckpoint_C" (`self.Interactable Checkpoint`) "Nutze die erhaltene Glyphe, um den Dash freizuschalten."))
      (`/Game/QuestSystem/Objectives/BP_ObjCollection.AddObjective` (`local.RootObjCollection`) _returnvalue_6 null))
    (:`then_6`
      (bind _returnvalue_7 (`|GenericCreateObject` "/Game/QuestSystem/Objectives/BP_ObjRechDestination.BP_ObjRechDestination_C" (`self.Flugschiff`) "Nutze dein Schiff, um die INsel zu verlassen."))
      (`/Game/QuestSystem/Objectives/BP_ObjCollection.AddObjective` (`local.RootObjCollection`) _returnvalue_7 null))))

(fn `UserConstructionScript`
  (`parent.UserConstructionScript`))