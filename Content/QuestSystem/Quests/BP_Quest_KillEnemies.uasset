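; Quest Blueprint that defines a "Kill Enemies" quest within the quest system.
; It constructs an order-required root objective collection, then adds a single kill-X-enemies objective to it.
; That objective takes its targets from the EnemiesToKill variable and a hardcoded kill count, while the NPC inputs go unused.
; The event graph holds no active logic.
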(fn `ConstructRootObjectiveCollection`
  (returns (RootObjCollection :type "/Game/QuestSystem/Objectives/BP_ObjCollection Object Reference"))
  (bind _returnvalue (`|GenericCreateObject` "/Game/QuestSystem/Objectives/BP_ObjCollection.BP_ObjCollection_C" true "Kill Enemies"))
  (return _returnvalue))

(fn `PopulateObjectives`
  (params (RootObjCollection :type "/Game/QuestSystem/Objectives/BP_ObjCollection Object Reference") (`NPC 1` :type "/Game/Blueprints/NPC/BP_NPC Object Reference") (`NPC 2` :type "/Game/Blueprints/NPC/BP_NPC Object Reference"))
  (bind _returnvalue (`|GenericCreateObject` "/Game/QuestSystem/Objectives/BP_ObjKillXEnemies.BP_ObjKillXEnemies_C" (`self.Enemies to Kill`) 4 "Kill x"))
  (bind _output_get (set `self.QuestObj` _returnvalue))
  (`/Game/QuestSystem/Objectives/BP_ObjCollection.AddObjective` (`local.RootObjCollection`) _output_get null self))

(fn `UserConstructionScript`
  (`parent.UserConstructionScript`))