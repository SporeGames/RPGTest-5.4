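; BP_Quest_Tutorial1 is a tutorial quest that has the player unlock the dash at a glyph, then board the ship to leave the island.
; It constructs an order-required root objective collection and fills it with an interact-with-checkpoint objective and a reach-destination objective.
; These objectives target the InteractableCheckpoint and Flugschiff references and carry hard-coded German display text.
; The event graph holds no active logic.
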(fn `ConstructRootObjectiveCollection`
  (returns (RootObjCollection :type "/Game/QuestSystem/Objectives/BP_ObjCollection Object Reference"))
  (bind _returnvalue (`|GenericCreateObject` "/Game/QuestSystem/Objectives/BP_ObjCollection.BP_ObjCollection_C" true "Stärke dich bevor du die Insel verlässt!"))
  (return _returnvalue))

(fn `PopulateObjectives`
  (params (RootObjCollection :type "/Game/QuestSystem/Objectives/BP_ObjCollection Object Reference") (NPC :type "/Game/Blueprints/NPC/BP_NPC Object Reference"))
  (`|ExecutionSequence`
    (:`then_0`
      (bind _returnvalue (`|GenericCreateObject` "/Game/QuestSystem/Objectives/BP_ObjInteractWithCheckpoint.BP_ObjInteractWithCheckpoint_C" (`self.Interactable Checkpoint`) "Nutze die Glyphe, um den Dash freizuschalten."))
      (`/Game/QuestSystem/Objectives/BP_ObjCollection.AddObjective` (`local.RootObjCollection`) _returnvalue null))
    (:`then_1`
      (bind _returnvalue_2 (`|GenericCreateObject` "/Game/QuestSystem/Objectives/BP_ObjRechDestination.BP_ObjRechDestination_C" (`self.Flugschiff`) "Betritt dein Schiff und verlasse die Insel."))
      (`/Game/QuestSystem/Objectives/BP_ObjCollection.AddObjective` (`local.RootObjCollection`) _returnvalue_2 null))))

(fn `UserConstructionScript`
  (`parent.UserConstructionScript`))