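; Killzone is a hazard actor that damages actors tagged "Damagable" when they overlap its Box component.
; Overlap starts a fast looping timer that repeatedly sends TakeDMG interface messages to the overlapping actor, with heavier damage for the player character.
; The timer stops on corruption limits, full for the player and depleted for others, with no end-overlap handling.
; A single timer handle is stored, so each new overlap overwrites it.
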(event `self.Box.OnComponentBeginOverlap`
  (params (OverlappedComponent :type "PrimitiveComponent Object Reference") (OtherActor :type "Actor Object Reference") (OtherComp :type "PrimitiveComponent Object Reference") (OtherBodyIndex :type Integer) (bFromSweep :type Boolean) (SweepResult :type "HitResult Structure (by ref)"))
  (if (`self.ActorHasTag` OtherActor "Damagable")
    (bind _returnvalue (`KismetSystemLibrary.K2_SetTimerDelegate` (delegate `Deal Dmage`) 0.05 true))
    (set `self.Damage Toimer` _returnvalue)))

(event `Deal Dmage`
  (if (== (`GameplayStatics.GetPlayerCharacter` 0) (stale `self.Box.OnComponentBeginOverlap` OtherActor))
    (bind _currentcorruption (message `/Game/Blueprints/BPI_Player.GetCurrentCorruption` (`GameplayStatics.GetPlayerCharacter` 0)))
    (if (>= _currentcorruption 100.0)
      (`KismetSystemLibrary.K2_ClearAndInvalidateTimerHandle` (`self.Damage Toimer`))
      (else
        (message `/Game/Blueprints/Enemies/BPI_Damagable.Take DMG` (stale `self.Box.OnComponentBeginOverlap` OtherActor) 5.0)))
    (else
      (bind _currentcorruption_2 (message `/Game/Blueprints/Enemies/BPI_Enemy.GetCurrentCorruption` (stale `self.Box.OnComponentBeginOverlap` OtherActor)))
      (if (<= _currentcorruption_2 0.0)
        (`KismetSystemLibrary.K2_ClearAndInvalidateTimerHandle` (`self.Damage Toimer`))
        (else
          (message `/Game/Blueprints/Enemies/BPI_Damagable.Take DMG` (stale `self.Box.OnComponentBeginOverlap` OtherActor) 1.5))))))

(fn `UserConstructionScript`)