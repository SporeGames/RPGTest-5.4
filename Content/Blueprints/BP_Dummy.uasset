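; BP_Dummy is a hittable dummy character that reacts to damage and can be knocked apart and reset.
; AnyDamage plays a random hit montage, while TakeDMG triggers a hit event that switches both static meshes to physics and turns off capsule collision.
; After a delay, it restores the transforms saved at BeginPlay and re-enables capsule collision.
; Health bar, health decrease, launch and respawn logic is unconnected, and GetStats returns zero.
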(event `self.ReceiveBeginPlay`
  (set `self.ActorTransform` (`self.GetTransform`))
  (set `self.StaticMeshTransform` (`SceneComponent.K2_GetComponentToWorld` (`self.StaticMesh`)))
  (set `self.StaticMesh1Transform_0` (`SceneComponent.K2_GetComponentToWorld` (`self.StaticMesh1`))))

(event `self.ReceiveTick`
  (params (DeltaSeconds :type "Float (single-precision)")))

(event `self.ReceiveAnyDamage`
  (params (Damage :type "Float (single-precision)") (DamageType :type "DamageType Object Reference") (InstigatedBy :type "Controller Object Reference") (DamageCauser :type "Actor Object Reference"))
  (`self.PlayAnimMontage` (`|GetArrayItem` (`self.hitAnims`) (`KismetMathLibrary.RandomIntegerInRange` 0 (- (`KismetArrayLibrary.Array_Length` (`self.hitAnims`)) 1))))
  (cast `/Game/ThirdPerson/Blueprints/BP_ThirdPersonCharacter` (`GameplayStatics.GetPlayerCharacter` 0)))

(event `/Game/Blueprints/Enemies/BPI_Damagable.Take DMG`
  (params (`DMG amount` :type "Float (double-precision)") (`Play Hit Reaction` :type Boolean) (`DMG Type` :type "/Game/Blueprints/Enemies/E_DMG_Type Enum" :default "NewEnumerator0"))
  (`KismetSystemLibrary.PrintString` "damage" :!enabledstate Disabled)
  (`self.OnHit`)
  (`self.HitEvent`))

(event `HitEvent`
  (bind _staticmesh (`self.StaticMesh`))
  (bind _staticmesh1 (`self.StaticMesh1`))
  (`PrimitiveComponent.SetSimulatePhysics` _staticmesh1 true)
  (`PrimitiveComponent.SetSimulatePhysics` _staticmesh true)
  (`PrimitiveComponent.SetCollisionEnabled` _staticmesh "PhysicsOnly")
  (`PrimitiveComponent.SetCollisionEnabled` _staticmesh1 "PhysicsOnly")
  (`PrimitiveComponent.SetCollisionEnabled` (`self.Capsule`) "NoCollision")
  (`KismetSystemLibrary.Delay` 5.0)
  (`PrimitiveComponent.SetSimulatePhysics` (`self.StaticMesh1`) false)
  (`PrimitiveComponent.SetSimulatePhysics` (`self.StaticMesh`) false)
  (`PrimitiveComponent.SetCollisionEnabled` (`self.Capsule`) "QueryAndPhysics")
  (`self.K2_SetActorTransform` (`self.ActorTransform`))
  (`SceneComponent.K2_SetWorldTransform` (`self.StaticMesh`) (`self.StaticMeshTransform`) false false)
  (`SceneComponent.K2_SetWorldTransform` (`self.StaticMesh1`) (`self.StaticMesh1Transform_0`) false false))

(fn `Get Stats`
  (returns (`Max HP` :type "Float (double-precision)"))
  (return 0.0))

(fn `UserConstructionScript`)