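; SafeSphere is a safe-zone actor that triggers corruption removal on the player while they are inside it.
; Overlapping its Box with a "Player"-tagged actor messages player character 0 to begin removing corruption, using the configured decrease value and tick.
; Ending the overlap sends the end message with both values zeroed.
; The construction script sets the Box's world scale from SafeSphereScale.
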(event `self.ReceiveBeginPlay`)

(event `self.Box.OnComponentBeginOverlap`
  (params (OverlappedComponent :type "PrimitiveComponent Object Reference") (OtherActor :type "Actor Object Reference") (OtherComp :type "PrimitiveComponent Object Reference") (OtherBodyIndex :type Integer) (bFromSweep :type Boolean) (SweepResult :type "HitResult Structure (by ref)"))
  (if (`self.ActorHasTag` OtherActor "Player")
    (message `/Game/Blueprints/BPI_Player.BeginRemovingCorruption` (`GameplayStatics.GetPlayerCharacter` 0) (`self.CorruptionDecreaseValue`) (`self.RemoveTick`))))

(event `self.Box.OnComponentEndOverlap`
  (params (OverlappedComponent :type "PrimitiveComponent Object Reference") (OtherActor :type "Actor Object Reference") (OtherComp :type "PrimitiveComponent Object Reference") (OtherBodyIndex :type Integer))
  (if (`self.ActorHasTag` OtherActor "Player")
    (message `/Game/Blueprints/BPI_Player.EndRemovingCorruption` (`GameplayStatics.GetPlayerCharacter` 0) 0.0 0.0)))

(fn `UserConstructionScript`
  (`SceneComponent.SetWorldScale3D` (`self.Box`) (`self.SafeSphereScale`)))