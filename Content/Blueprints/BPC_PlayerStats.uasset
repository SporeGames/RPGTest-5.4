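; Actor component that tracks health, stamina, XP and level for the player character, and also serves BP_Dummy actors.
; On BeginPlay it identifies its owner; health damage updates either the player HUD or dummy health bar and reports depletion.
; Other stat functions write directly to the player HUD.
; Reaching max XP raises the level and XP cap, resets XP, then opens WB_PausMenu with the game paused.
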(event `self.ReceiveBeginPlay`
  (`KismetSystemLibrary.DelayUntilNextTick`)
  (bind _asbp_third_person_character (cast `/Game/ThirdPerson/Blueprints/BP_ThirdPersonCharacter` (`self.GetOwner`))
    (:`then`
      (set `self.Player Character BP` _asbp_third_person_character)
      (set `self.isPlayer` true)
      (`self.SetHUD`))
    (:`CastFailed`
      (bind _asbp_dummy (cast `/Game/Blueprints/BP_Dummy` (`self.GetOwner`)))
      (set `self.DummyBP` _asbp_dummy)
      (set `self.isPlayer` false))))

(event `SetHUD`
  (`KismetSystemLibrary.DelayUntilNextTick`)
  (`ProgressBar.SetPercent` (`/Game/UI/WB_HUD.XPBar` (`/Game/ThirdPerson/Blueprints/BP_ThirdPersonCharacter.HudWidget` (`self.Player Character BP`))) (/ (`self.XP`) (`self.MaxXP`)))
  (`TextBlock.SetText` (`/Game/UI/WB_HUD.LevelTxt` (`/Game/ThirdPerson/Blueprints/BP_ThirdPersonCharacter.HudWidget` (`self.Player Character BP`))) (`KismetTextLibrary.Conv_IntToText` (`self.Level`)))
  (`ProgressBar.SetPercent` (select `bool` (`self.isPlayer`) :`false` (`/Game/UI/WB_DummyHealthBar.HealthBar` (`/Game/Blueprints/BP_Dummy.HealthBarUI` (`self.DummyBP`))) :`true` (`/Game/UI/WB_HUD.HealthBar` (`/Game/ThirdPerson/Blueprints/BP_ThirdPersonCharacter.HudWidget` (`self.Player Character BP`)))) (/ (`self.CurrentHealth`) (`self.MaxHealth`))))

(event `LevelUP`
  (bind _returnvalue (`GameplayStatics.GetPlayerController` 0))
  (bind _returnvalue_2 (`|CreateWidget` "/Game/UI/WB_PausMenu.WB_PausMenu_C"))
  (`UserWidget.AddToViewport` _returnvalue_2 0)
  (`GameplayStatics.SetGamePaused` true)
  (set `PlayerController.bShowMouseCursor` true _returnvalue)
  (`WidgetBlueprintLibrary.SetInputMode_GameAndUIEx` _returnvalue _returnvalue_2))

(fn `DecraseStamina`
  (params (StaminaDecrease :type "Float (double-precision)"))
  (returns (NoStaminaLeft :type Boolean))
  (if (not (<= (`self.CurrentStamina`) 0.0))
    (set `self.CurrentStamina` (- (`self.CurrentStamina`) StaminaDecrease))
    (`ProgressBar.SetPercent` (`/Game/UI/WB_HUD.StaminaBar` (`/Game/ThirdPerson/Blueprints/BP_ThirdPersonCharacter.HudWidget` (`self.Player Character BP`))) (/ (`self.CurrentStamina`) (`self.MaxStamina`)))
    (if (<= (`self.CurrentStamina`) 0.0)
      (return true)
      (else
        (return false)))
    (else
      (return true))))

(fn `Decrease Health`
  (params (Damage :type "Float (double-precision)"))
  (returns (IsPlayerDead :type Boolean))
  (if (not (<= (`self.CurrentHealth`) 0.0))
    (bind _output_get (set `self.CurrentHealth` (- (`self.CurrentHealth`) Damage)))
    (`ProgressBar.SetPercent` (select `bool` (`self.isPlayer`) :`false` (`/Game/UI/WB_DummyHealthBar.HealthBar` (`/Game/Blueprints/BP_Dummy.HealthBarUI` (`self.DummyBP`))) :`true` (`/Game/UI/WB_HUD.HealthBar` (`/Game/ThirdPerson/Blueprints/BP_ThirdPersonCharacter.HudWidget` (`self.Player Character BP`)))) (/ _output_get (`self.MaxHealth`)))
    (if (<= (`self.CurrentHealth`) 0.0)
      (return true)
      (else
        (return false)))
    (else
      (return true))))

(fn `IncreaseHealth`
  (params (AddedHealth :type "Float (double-precision)"))
  (set `self.CurrentHealth` (+ (`self.CurrentHealth`) AddedHealth))
  (if (> (`self.CurrentHealth`) (`self.MaxHealth`))
    (set `self.CurrentHealth` (`self.MaxHealth`)))
  (`ProgressBar.SetPercent` (`/Game/UI/WB_HUD.HealthBar` (`/Game/ThirdPerson/Blueprints/BP_ThirdPersonCharacter.HudWidget` (`self.Player Character BP`))) (/ (`self.CurrentHealth`) (`self.MaxHealth`))))

(fn `IncreaseLevel`
  (params (AddedLevel :type Integer))
  (set `self.Level` (+ (`self.Level`) AddedLevel))
  (set `self.MaxXP` (+ (`self.MaxXP`) 150.0))
  (set `self.XP` 0.0)
  (`TextBlock.SetText` (`/Game/UI/WB_HUD.LevelTxt` (`/Game/ThirdPerson/Blueprints/BP_ThirdPersonCharacter.HudWidget` (`self.Player Character BP`))) (`KismetTextLibrary.Conv_IntToText` (`self.Level`)))
  (`self.LevelUP`))

(fn `IncreaseMaxHealth`
  (params (HealthIncremention :type "Float (double-precision)"))
  (set `self.MaxHealth` (+ (`self.MaxHealth`) HealthIncremention))
  (`ProgressBar.SetPercent` (`/Game/UI/WB_HUD.HealthBar` (`/Game/ThirdPerson/Blueprints/BP_ThirdPersonCharacter.HudWidget` (`self.Player Character BP`))) (/ (`self.CurrentHealth`) (`self.MaxHealth`))))

(fn `IncreaseMaxStamina`
  (params (AddedStamina :type "Float (double-precision)"))
  (set `self.MaxStamina` (+ (`self.MaxStamina`) AddedStamina))
  (`ProgressBar.SetPercent` (`/Game/UI/WB_HUD.StaminaBar` (`/Game/ThirdPerson/Blueprints/BP_ThirdPersonCharacter.HudWidget` (`self.Player Character BP`))) (/ (`self.CurrentStamina`) (`self.MaxStamina`))))

(fn `IncreaseStamina`
  (params (AddedStamina :type "Float (double-precision)"))
  (set `self.CurrentStamina` (+ (`self.CurrentStamina`) AddedStamina))
  (if (> (`self.CurrentStamina`) (`self.MaxStamina`))
    (set `self.CurrentStamina` (`self.MaxStamina`)))
  (`ProgressBar.SetPercent` (`/Game/UI/WB_HUD.StaminaBar` (`/Game/ThirdPerson/Blueprints/BP_ThirdPersonCharacter.HudWidget` (`self.Player Character BP`))) (/ (`self.CurrentStamina`) (`self.MaxStamina`))))

(fn `IncreaseXP`
  (params (AddedXP :type "Float (double-precision)"))
  (set `self.XP` (+ (`self.XP`) AddedXP))
  (if (>= (`self.XP`) (`self.MaxXP`))
    (`self.IncreaseLevel` 1))
  (`ProgressBar.SetPercent` (`/Game/UI/WB_HUD.XPBar` (`/Game/ThirdPerson/Blueprints/BP_ThirdPersonCharacter.HudWidget` (`self.Player Character BP`))) (/ (`self.XP`) (`self.MaxXP`))))