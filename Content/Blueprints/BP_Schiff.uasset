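; BP_Schiff is an actor that moves its ship component (Schiff) along a spline when play begins.
; A Timeline, with play rate scaled by TimeToCompleteInSeconds, drives an alpha that is lerped across the spline length.
; Each update places the ship at that distance in world space, following the spline's rotation with a -90 degree yaw offset to correct its facing.
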(event `self.ReceiveBeginPlay`
  (bind _spline (`self.Spline`))
  (`TimelineComponent.SetPlayRate` (`self.Timeline`) (/ 1.0 (`self.Time to Complete in Seconds`)))
  (bind (_direction _alpha) (`Timeline|Timeline` :!via `PlayFromStart`)
    (:`Update`
      (bind _returnvalue (`SplineComponent.GetTransformAtDistanceAlongSpline` _spline (`KismetMathLibrary.Lerp` 0.0 (`SplineComponent.GetSplineLength` _spline) _alpha) "World" false))
      (`SceneComponent.K2_SetWorldTransform` (`self.Schiff`) (`KismetMathLibrary.MakeTransform` (.location _returnvalue) (`KismetMathLibrary.MakeRotator` (.roll (.rotation _returnvalue)) (.pitch (.rotation _returnvalue)) (+ (.yaw (.rotation _returnvalue)) -90.0))) false false))))

(fn `UserConstructionScript`)