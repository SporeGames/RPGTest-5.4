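; Destructible flower pot (Blumentopf) actor that reacts to being destroyed or hit by physics.
; Destructed and HitbyPhysic share one DoOnce, so the break response runs a single time.
; It plays the TopfExplosion audio event at the actor's location and destroys the StaticMesh component, leaving the actor itself in place.
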(event `self.Destructed`
  (`/Engine/EditorBlueprintResources/StandardMacros.DoOnce` false :!label _label
    (:`Completed`
      (`FMODBlueprintStatics.PlayEventAtLocation` "/Game/FMOD/Events/TopfExplosion.TopfExplosion" (`KismetMathLibrary.MakeTransform` (`self.K2_GetActorLocation`)))
      (`ActorComponent.K2_DestroyComponent` (`self.StaticMesh`)))))

(event `self.HitByPhysic`
  (params (`Hit Location` :type "Vector Structure"))
  (goto _label))

(fn `UserConstructionScript`
  (`parent.UserConstructionScript`))