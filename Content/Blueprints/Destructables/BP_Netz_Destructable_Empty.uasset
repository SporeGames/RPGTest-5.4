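; Destructible net actor, built on a Geometry Collection, that plays audio and camera feedback as it tears and drops.
; On BeginPlay it plays a tearing event, waits briefly, then traces downward and fires two staggered pumpkin-explosion events at the ground impact point.
; The collection's first component hit triggers, once only, a world camera shake and a barrel-explosion event.
; Chaos break handlers are empty, and the master-field spawn logic is unconnected.
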(event `self.ReceiveBeginPlay`
  (bind (_returnvalue_x _returnvalue_y) (`KismetMathLibrary.BreakVector` (`self.K2_GetActorLocation`)))
  (`FMODBlueprintStatics.PlayEventAtLocation` "/Game/FMOD/Events/Reißen.Reißen" (`KismetMathLibrary.MakeTransform` (`self.K2_GetActorLocation`)))
  (`KismetSystemLibrary.Delay` 0.8)
  (bind _outhit (`KismetSystemLibrary.LineTraceSingle` (`self.K2_GetActorLocation`) (`KismetMathLibrary.MakeVector` _returnvalue_x _returnvalue_y -1000.0) "TraceTypeQuery1"))
  (bind (_bblockinghit _binitialoverlap _time _distance _location _impactpoint) (`GameplayStatics.BreakHitResult` _outhit))
  (`FMODBlueprintStatics.PlayEventAtLocation` "/Game/FMOD/Events/KürbisExplosion.KürbisExplosion" (`KismetMathLibrary.MakeTransform` _impactpoint))
  (`KismetSystemLibrary.Delay` 0.1)
  (`FMODBlueprintStatics.PlayEventAtLocation` "/Game/FMOD/Events/KürbisExplosion.KürbisExplosion" (`KismetMathLibrary.MakeTransform` _impactpoint)))

(event `self.GeometryCollection.OnChaosBreakEvent`
  (params (BreakEvent :type "ChaosBreakEvent Structure (by ref)")))

(event `self.GeometryCollection.OnChaosCrumblingEvent`
  (params (CrumbleEvent :type "ChaosCrumblingEvent Structure (by ref)")))

(event `self.GeometryCollection.OnChaosPhysicsCollision`
  (params (CollisionInfo :type "ChaosPhysicsCollisionInfo Structure (by ref)")))

(event `self.GeometryCollection.OnComponentHit`
  (params (HitComponent :type "PrimitiveComponent Object Reference") (OtherActor :type "Actor Object Reference") (OtherComp :type "PrimitiveComponent Object Reference") (NormalImpulse :type "Vector Structure") (Hit :type "HitResult Structure (by ref)"))
  (`/Engine/EditorBlueprintResources/StandardMacros.DoOnce` false
    (:`Completed`
      (`GameplayStatics.PlayWorldCameraShake` "/Game/Art/Enviroment/Deko/SS_ChaosHitGround.SS_ChaosHitGround_C" (`self.K2_GetActorLocation`) 0.0 2000.0 1.0 true)
      (`FMODBlueprintStatics.PlayEventAtLocation` "/Game/FMOD/Events/BarrelExplosion_2.BarrelExplosion_2" (`KismetMathLibrary.MakeTransform` (`SceneComponent.K2_GetComponentLocation` (`self.GeometryCollection`)))))))

(fn `UserConstructionScript`)