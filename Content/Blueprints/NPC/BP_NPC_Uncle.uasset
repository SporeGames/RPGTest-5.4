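; BP_NPC_Uncle is an NPC Blueprint that walks the uncle character along a hardcoded route of destination actors.
; Its HardcodeMoveTO event waits briefly, then runs AI Move To toward the actor at the current index in the Destination array.
; Each successful move increments the index and loops until the array is exhausted; failed moves are not handled, and nothing in this Blueprint calls the event.
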(event `HardcodeMoveTO`
  (`KismetSystemLibrary.Delay` 3.0)
  (`|AIMoveTo` self (`self.K2_GetActorLocation` (`|GetArrayItem` (`self.Destination`) (`self.Inde`))) null :!label _label
    (:`OnSuccess`
      (bind _result (`/Engine/EditorBlueprintResources/StandardMacros.IncrementInt` (`self.Inde`))
        (:`  `
          (set `self.Inde` _result)
          (if (> (`KismetArrayLibrary.Array_Length` (`self.Destination`)) (`self.Inde`))
            (goto _label)))))))

(fn `UserConstructionScript`
  (`parent.UserConstructionScript`))