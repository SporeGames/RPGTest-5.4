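; Mother NPC Blueprint that walks through an ordered array of destination actors.
; The HardcodeMoveTO event prints the current target location, waits briefly, then chains AI MoveTo calls, advancing the index on each success until the array ends.
; A failed move prints a debug message and stops the chain.
; Nothing in this Blueprint calls the event, and BeginPlay only holds a disabled parent call.
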(event `HardcodeMoveTO`
  (bind _returnvalue (`self.K2_GetActorLocation` (`|GetArrayItem` (`self.Destination`) (`self.Index`))))
  (`KismetSystemLibrary.PrintString` (`KismetStringLibrary.Conv_VectorToString` _returnvalue))
  (`KismetSystemLibrary.Delay` 5.0)
  (`|AIMoveTo` self _returnvalue null :!label _label
    (:`OnSuccess`
      (bind _result (`/Engine/EditorBlueprintResources/StandardMacros.IncrementInt` (`self.Index`))
        (:`  `
          (set `self.Index` _result)
          (if (> (`KismetArrayLibrary.Array_Length` (`self.Destination`)) (`self.Index`))
            (goto _label)))))
    (:`OnFail`
      (`KismetSystemLibrary.PrintString` "FAILFAILFAIl"))))

(fn `UserConstructionScript`
  (`parent.UserConstructionScript`))