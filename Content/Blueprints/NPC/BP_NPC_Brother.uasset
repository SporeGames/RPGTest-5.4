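; BP_NPC_Brother is an NPC that walks a fixed route through an ordered array of destination actors.
; The HardcodeMoveTO event waits briefly, then chains AI Move To calls, advancing the index after each success until the array ends.
; At the last stop, it snaps to the rotation of that destination's Arrow.
; The event is not triggered within this Blueprint, and failed moves are not handled.
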(event `HardcodeMoveTO`
  (`KismetSystemLibrary.Delay` 3.0)
  (`|AIMoveTo` self (`self.K2_GetActorLocation` (`|GetArrayItem` (`self.Destination`) (`self.Index`))) null :!label _label
    (:`OnSuccess`
      (bind _result (`/Engine/EditorBlueprintResources/StandardMacros.IncrementInt` (`self.Index`))
        (:`  `
          (set `self.Index` _result)
          (if (> (`KismetArrayLibrary.Array_Length` (`self.Destination`)) (`self.Index`))
            (goto _label)
            (else
              (`self.K2_SetActorRotation` (`SceneComponent.K2_GetComponentRotation` (`/Game/Blueprints/NPC/BP_PatrolObject.Arrow` (`|GetArrayItem` (`self.Destination`) (- (`self.Index`) 1))))))))))))

(fn `UserConstructionScript`
  (`parent.UserConstructionScript`))