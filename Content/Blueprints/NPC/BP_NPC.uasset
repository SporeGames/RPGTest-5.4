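; BP_NPC is an AI-controlled NPC character that switches between idle and interaction states.
; BeginPlay and the two state events set the NPCStates enum and copy it to the AI controller's Blackboard "State" key, starting in idle.
; A separate event sets the walk speed.
; LookAtPlayer only prints a debug string, as its rotate-toward-player nodes are left disconnected.
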(event `self.ReceiveBeginPlay`
  (set `self.NPCStates` "NewEnumerator0")
  (`BlackboardComponent.SetValueAsEnum` (`AIBlueprintHelperLibrary.GetBlackboard` (`AIBlueprintHelperLibrary.GetAIController` self)) "State" (`self.NPCStates`)))

(event `/Game/Blueprints/NPC/BPI_NPC.ChangeMovmentSpeed`
  (params (Speed :type "Float (double-precision)"))
  (set `CharacterMovementComponent.MaxWalkSpeed` Speed (`self.CharacterMovement`)))

(event `LookAtPlayer`
  (`KismetSystemLibrary.PrintString` "Rotation"))

(event `/Game/Blueprints/NPC/BPI_NPC.StateIdle`
  (set `self.NPCStates` "NewEnumerator0")
  (`BlackboardComponent.SetValueAsEnum` (`AIBlueprintHelperLibrary.GetBlackboard` (`AIBlueprintHelperLibrary.GetAIController` self)) "State" (`self.NPCStates`)))

(event `/Game/Blueprints/NPC/BPI_NPC.StateInteraction`
  (set `self.NPCStates` "NewEnumerator1")
  (`BlackboardComponent.SetValueAsEnum` (`AIBlueprintHelperLibrary.GetBlackboard` (`AIBlueprintHelperLibrary.GetAIController` self)) "State" (`self.NPCStates`))
  (`KismetSystemLibrary.PrintString` "CHANGE STATE"))

(fn `UserConstructionScript`)