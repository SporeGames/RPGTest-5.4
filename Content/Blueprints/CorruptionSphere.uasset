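; Corruption zone actor that notifies the player character of corruption when a Player-tagged actor enters or leaves its Box volume.
; Overlap begin passes the corruption value and tick rate to the character, and overlap end sends zeroed reset values.
; From BeginPlay, a timer spawns random Niagara effects in the box, using vertical traces to place them above the surface, plus a firefly system with no location set.
; The player-following particle timer is disconnected.
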(event `Spawn Particle`
  (`NiagaraFunctionLibrary.SpawnSystemAtLocation` "/Game/Art/Particle/CorruptionZoneEffect/NS_Corruption_V2.NS_Corruption_V2" (`self.K2_GetActorLocation` (`GameplayStatics.GetPlayerCharacter` 0))))

(event `self.Box.OnComponentBeginOverlap`
  (params (OverlappedComponent :type "PrimitiveComponent Object Reference") (OtherActor :type "Actor Object Reference") (OtherComp :type "PrimitiveComponent Object Reference") (OtherBodyIndex :type Integer) (bFromSweep :type Boolean) (SweepResult :type "HitResult Structure (by ref)"))
  (if (`self.ActorHasTag` OtherActor "Player")
    (set `self.Looping` true)
    (message `/Game/Blueprints/BPI_Player.BeginCorruption` (`GameplayStatics.GetPlayerCharacter` 0) (`self.Corruption`) (`self.TickRate`))))

(event `self.Box.OnComponentEndOverlap`
  (params (OverlappedComponent :type "PrimitiveComponent Object Reference") (OtherActor :type "Actor Object Reference") (OtherComp :type "PrimitiveComponent Object Reference") (OtherBodyIndex :type Integer))
  (if (`self.ActorHasTag` OtherActor "Player")
    (set `self.Looping` false)
    (message `/Game/Blueprints/BPI_Player.EndCorruption` (`GameplayStatics.GetPlayerCharacter` 0) 0.0 0.0)))

(event `self.ReceiveBeginPlay`
  (`self.Spawn Particles Loop`)
  (`KismetSystemLibrary.PrintText` "Hello"))

(event `Spawn Particles Loop`
  (`KismetSystemLibrary.K2_SetTimerDelegate` (delegate `SpawnParticles`) (`self.Time`) (`self.Looping_0`)))

(event `SpawnParticles`
  (bind (_returnvalue_x _returnvalue_y _returnvalue_z) (`KismetMathLibrary.BreakVector` (`BoxComponent.GetScaledBoxExtent` (`self.Box`))))
  (for _ (range 4)
    (bind _output_get (set `self.SetVector` (`KismetMathLibrary.MakeVector` (`KismetMathLibrary.RandomFloatInRange` (* _returnvalue_y -1.0) _returnvalue_y) (`KismetMathLibrary.RandomFloatInRange` (* _returnvalue_x -1.0) _returnvalue_x) (`KismetMathLibrary.RandomFloatInRange` (* _returnvalue_z -1.0) _returnvalue_z))))
    (bind (_returnvalue_x_2 _returnvalue_y_2 _returnvalue_z_2) (`KismetMathLibrary.BreakVector` (+ _output_get (`SceneComponent.K2_GetComponentLocation` (`self.Box`)))))
    (bind _outhit (`KismetSystemLibrary.LineTraceSingle` (`KismetMathLibrary.MakeVector` _returnvalue_x_2 _returnvalue_y_2 (+ _returnvalue_z_2 1000.0)) (`KismetMathLibrary.MakeVector` _returnvalue_x_2 _returnvalue_y_2 (+ _returnvalue_z_2 -1000.0)) "TraceTypeQuery1"))
    (bind (_bblockinghit _binitialoverlap _time _distance _location _impactpoint) (`GameplayStatics.BreakHitResult` _outhit))
    (`NiagaraFunctionLibrary.SpawnSystemAtLocation` (`KismetArrayLibrary.Array_Random` (`self.Particle`)) (`KismetMathLibrary.MakeVector` (.x _impactpoint) (.y _impactpoint) (+ (.z _impactpoint) (`KismetMathLibrary.RandomFloatInRange` 50.0 300.0))))
    (`NiagaraFunctionLibrary.SpawnSystemAtLocation` "/Game/Art/Particle/CorruptionDebuff/NS_CorruptionZoneFireflys.NS_CorruptionZoneFireflys")))

(fn `UserConstructionScript`)