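; Boomerang projectile actor that flies out along its forward vector on spawn, returns to the player and destroys itself.
; Two timelines lerp its location: a swept outbound leg, cut short by environment hits, and an unswept return tracking the player's current position.
; Overlaps with "Damagable" actors deal damage, shorten the player's dash cooldown and shake the camera.
; Sound events cover throw, looping flight, impacts, return and catch.
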(event `Throw_Var_1`
  (bind _returnvalue (+ (`self.K2_GetActorLocation`) (* (`self.GetActorForwardVector`) (`self.Distance`))))
  ;[1 1 1] Hinweg
  ;;[0.08333 0.08333 0.08333] Boomerang Loop Sound
  (`FMODBlueprintStatics.PlayEvent2D` "/Game/FMOD/Events/BoomerangWurf.BoomerangWurf")
  (`KismetSystemLibrary.K2_SetTimerDelegate` (delegate `Loop Sound Hinweg`) 0.25 true true)
  (set `self.Start Location` (`self.K2_GetActorLocation`))
  (set `self.Goal Location` _returnvalue)
  (`KismetSystemLibrary.SphereTraceSingle` :`Start` _returnvalue :`End` _returnvalue :`Radius` 15.0 :`TraceChannel` "TraceTypeQuery1" :`DrawDebugType` "ForDuration")
  (bind (_direction _alpha) (`Timeline|Hinweg` :!via `PlayFromStart` :!label _label)
    (:`Update`
      ;;[1 1 1] Sweep needs to be on or else not get hit by environment
      (`self.K2_SetActorLocation` (`KismetMathLibrary.VLerp` (`self.Start Location`) (`self.Goal Location`) _alpha) true))
    (:`Finished`
      (`KismetSystemLibrary.Delay` (`self.WaitTime`))
      (`FMODBlueprintStatics.PlayEventAtLocation` "/Game/FMOD/Events/Boomerang_Flyback.Boomerang_Flyback" (`KismetMathLibrary.MakeTransform` (`self.K2_GetActorLocation`)))
      (`self.Fly Rückweg`))))

(event `Loop Sound Hinweg`
  ;[1 1 1] Hinweg
  ;;[0.08333 0.08333 0.08333] Boomerang Loop Sound
  (`FMODBlueprintStatics.PlayEventAtLocation` "/Game/FMOD/Events/BoomerangFlight.BoomerangFlight" (`KismetMathLibrary.MakeTransform` (`self.K2_GetActorLocation`))))

(event `Stop Hinweg`
  ;[1 1 1] Hinweg
  (`FMODBlueprintStatics.PlayEventAtLocation` "/Game/FMOD/Events/BoomerangHitEnvironment.BoomerangHitEnvironment" (`KismetMathLibrary.MakeTransform` (`self.K2_GetActorLocation`)))
  (`|ExecutionSequence`
    (:`then_0`
      (goto _label :!via `Stop`))
    (:`then_1`
      (set `self.Goal Location` (`self.K2_GetActorLocation`))
      (`KismetSystemLibrary.Delay` 0.2)
      (`self.Fly Rückweg`))))

(event `self.ReceiveBeginPlay`
  (`self.Throw_Var_1`))

(event `Fly Rückweg`
  (bind _returnvalue (`GameplayStatics.GetPlayerCharacter` 0))
  ;[1 1 1] Rückweg
  (set `self.OnRückweg` true)
  (bind (_direction _alpha) (`Timeline|Rückweg`)
    (:`Update`
      (`self.K2_SetActorLocation` (`KismetMathLibrary.VLerp` (`self.Goal Location`) (`self.K2_GetActorLocation` (`GameplayStatics.GetPlayerCharacter` 0)) _alpha)))
    (:`Finished`
      (message `/Game/Blueprints/BPI_Player.BoomerangArrivedAtPlayer` _returnvalue)
      (`FMODBlueprintStatics.PlayEventAtLocation` "/Game/FMOD/Events/BoomerangCatch.BoomerangCatch" (`KismetMathLibrary.MakeTransform` (`self.K2_GetActorLocation` _returnvalue)))
      (`self.K2_DestroyActor`))))

(event `self.Hitbox.OnComponentBeginOverlap`
  (params (OverlappedComponent :type "PrimitiveComponent Object Reference") (OtherActor :type "Actor Object Reference") (OtherComp :type "PrimitiveComponent Object Reference") (OtherBodyIndex :type Integer) (bFromSweep :type Boolean) (SweepResult :type "HitResult Structure (by ref)"))
  ;[1 1 1] Enemies need Tag or sth to check
  (set `self.Hit Actor` OtherActor)
  (if (`self.ActorHasTag` (`self.Hit Actor`) "Damagable")
    (message `/Game/Blueprints/BPI_Player.ReduceDashCD` (`GameplayStatics.GetPlayerCharacter` 0) 0.2)
    (message `/Game/Blueprints/Enemies/BPI_Damagable.Take DMG` (`self.Hit Actor`) 1.0 false)
    (`GameplayStatics.PlayWorldCameraShake` "/Game/Blueprints/CC_BoomerangHit.CC_BoomerangHit_C" (`self.K2_GetActorLocation` (`GameplayStatics.GetPlayerCharacter` 0)) 0.0 1500.0 0.0)
    (`self.HitSound`)))

(event `HitSound`
  (bind _returnvalue (`KismetMathLibrary.MakeTransform` (`self.K2_GetActorLocation`)))
  ;[1 1 1] Hit Sound (SOUND DESIGN)
  (if (`self.ActorHasTag` (`self.Hit Actor`) "Dummy")
    (`FMODBlueprintStatics.PlayEventAtLocation` "/Game/FMOD/Events/DummyImpact.DummyImpact" _returnvalue)
    (else
      (`FMODBlueprintStatics.PlayEventAtLocation` "/Game/FMOD/Events/BoomerangHitEnemy.BoomerangHitEnemy" _returnvalue))))

(event `self.Hitbox.OnComponentHit`
  (params (HitComponent :type "PrimitiveComponent Object Reference") (OtherActor :type "Actor Object Reference") (OtherComp :type "PrimitiveComponent Object Reference") (NormalImpulse :type "Vector Structure") (Hit :type "HitResult Structure (by ref)"))
  (bind (_bblockinghit _binitialoverlap _time _distance _location _impactpoint _normal _impactnormal _physmat _hitactor _hitcomponent) (`GameplayStatics.BreakHitResult` Hit))
  ;[1 1 1] Environment Collision
  (`KismetSystemLibrary.PrintString` (`KismetSystemLibrary.GetDisplayName` _hitactor))
  (`KismetSystemLibrary.PrintString` (`KismetSystemLibrary.GetDisplayName` _hitcomponent))
  (set `self.Hit Actor` _hitactor)
  (`self.Stop Hinweg`))

(fn `UserConstructionScript`)