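; BP_Tritplatform is an interactable platform prop that drops when its HitbyPhysic event is triggered from outside its own graph.
; The event destroys the Box, turns on physics and gravity for the Cube, and releases the Cable's attached end.
; After a two-second delay, it stops simulating physics on the Cube and destroys the Kugel (ball) component.
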(event `self.ReceiveBeginPlay`)

(event `self.HitByPhysic`
  (params (`Hit Location` :type "Vector Structure"))
  (bind _cube (`self.Cube`))
  (`ActorComponent.K2_DestroyComponent` (`self.Box`))
  (`PrimitiveComponent.SetSimulatePhysics` _cube true)
  (`PrimitiveComponent.SetEnableGravity` _cube true)
  (set `CableComponent.bAttachEnd` false (`self.Cable`))
  (`KismetSystemLibrary.Delay` 2.0)
  (`PrimitiveComponent.SetSimulatePhysics` (`self.Cube`) false)
  (`ActorComponent.K2_DestroyComponent` (`self.Kugel`)))

(fn `UserConstructionScript`)