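; BP_Button_Crane is an interactable button, named for a crane, that triggers its linked ActorToInteract when used.
; On interaction it switches the player's input from the menu to the default mapping, sets walking movement and sends the interaction message to that actor.
; It then hides its child-actor interaction hint and slides the Cube with a duration-scaled Timeline, skipping both if the hint cast fails.
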(event `/Game/Blueprints/InteractionInterface.OnInteraction`
  (params (PlayerCharakter :type "/Game/ThirdPerson/Blueprints/BP_ThirdPersonCharacter Object Reference"))
  (message `/Game/Blueprints/BPI_Player.SetPlayerInput` PlayerCharakter "/Game/ThirdPerson/Input/IMC_Default.IMC_Default" "/Game/ThirdPerson/Input/IMC_Menu.IMC_Menu")
  (`CharacterMovementComponent.SetMovementMode` (`Character.CharacterMovement` (`GameplayStatics.GetPlayerCharacter` 0)) "MOVE_Walking" 0)
  (message `/Game/Blueprints/InteractionInterface.OnInteraction` (`self.ActorToInteract`) null)
  (bind _asbp_interaction_hint (cast `/Game/Blueprints/Interactables/BP_InteractionHint` (`ChildActorComponent.ChildActor` (`self.BP_InteractionHint`)))
    (:`then`
      (`/Game/Blueprints/Interactables/BP_InteractionHint.HideUIHint` _asbp_interaction_hint)
      (`TimelineComponent.SetPlayRate` (`self.Timeline`) (/ 1.0 (`self.Duration in Seconds`)))
      (bind (_direction _alpha) (`Timeline|Timeline` :!via `PlayFromStart`)
        (:`Update`
          (`SceneComponent.K2_SetRelativeLocation` (`self.Cube`) (`KismetMathLibrary.VLerp` (0.0 0.0 0.0) (10.0 0.0 0.0) _alpha) false false))))
    (:`CastFailed`
      (`KismetSystemLibrary.PrintString` "failed :("))))

(fn `UserConstructionScript`
  (`parent.UserConstructionScript`))