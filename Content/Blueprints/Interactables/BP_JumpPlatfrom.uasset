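; A breakable jump platform interactable with a barrel mesh, a ball (Kugel) and a cable.
; On its first HitbyPhysic event, it spawns BP_JumpPlatform_Destructable at the mesh's transform and destroys the intact mesh shortly after.
; It then enables gravity and physics on the ball and detaches the cable's end.
; After a delay, it destroys the box, ball and cable components.
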(event `self.ReceiveBeginPlay`)

(event `/Game/Blueprints/Interactables/BPI_PhysicInteraction.HitByPhysic`
  (params (`Hit Location` :type "Vector Structure"))
  (bind _kugel (`self.Kugel`))
  (bind _returnvalue (`SceneComponent.K2_GetComponentToWorld` (`self.SM_MERGED_BarrelJump`)))
  (set `self.Location` (`KismetMathLibrary.MakeVector` (.x (.location _returnvalue)) (.y (.location _returnvalue)) (.z (.location _returnvalue))))
  (`/Engine/EditorBlueprintResources/StandardMacros.DoOnce` false
    (:`Completed`
      (`|SpawnActorFromClass` "/Game/Blueprints/Destructables/BP_JumpPlatform_Destructable.BP_JumpPlatform_Destructable_C" (`KismetMathLibrary.MakeTransform` (`self.Location`) (.rotation _returnvalue) (.scale _returnvalue)) "AlwaysSpawn" "MultiplyWithRoot" null null)
      (`KismetSystemLibrary.Delay` 0.2)
      (`ActorComponent.K2_DestroyComponent` (`self.SM_MERGED_BarrelJump`))
      (`PrimitiveComponent.SetEnableGravity` _kugel true)
      (`PrimitiveComponent.SetSimulatePhysics` _kugel true)
      (set `CableComponent.bAttachEnd` false (`self.Cable`))
      (`KismetSystemLibrary.Delay` 5.0)
      (`ActorComponent.K2_DestroyComponent` (`self.Box`))
      (`ActorComponent.K2_DestroyComponent` (`self.Kugel`))
      (`ActorComponent.K2_DestroyComponent` (`self.Cable`)))))

(fn `UserConstructionScript`)