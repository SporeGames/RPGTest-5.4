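; Village item interactable that, on interaction, adds its configured quest to the player character's quest list if absent and is collected either way.
; Collection fires the interacted event, sets player input to the default mapping context while removing the menu one, and plays a 2D collect sound.
; It also shows a talking-zone widget with the item's text, set to destroy itself after a configurable delay.
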(event `/Game/Blueprints/InteractionInterface.OnInteraction`
  (params (PlayerCharakter :type "/Game/ThirdPerson/Blueprints/BP_ThirdPersonCharacter Object Reference"))
  (if (== (`KismetArrayLibrary.Array_Find` (`/Game/ThirdPerson/Blueprints/BP_ThirdPersonCharacter.Quests` PlayerCharakter) (`self.QuestToActiviate`)) -1)
    (`KismetArrayLibrary.Array_Add` (`/Game/ThirdPerson/Blueprints/BP_ThirdPersonCharacter.Quests` PlayerCharakter) (`self.QuestToActiviate`))
    (`self.CollectItem`)
    (else
      (`self.CollectItem`))))

(event `CollectItem`
  (`self.OnInteracted`)
  (`/Game/ThirdPerson/Blueprints/BP_ThirdPersonCharacter.SetPlayerInput` (stale `/Game/Blueprints/InteractionInterface.OnInteraction` PlayerCharakter) "/Game/ThirdPerson/Input/IMC_Default.IMC_Default" "/Game/ThirdPerson/Input/IMC_Menu.IMC_Menu")
  (`self.CreateWidget`)
  ;[0.6 0.2598 1] Kim Sound (Item Collect)
  (`FMODBlueprintStatics.PlayEvent2D` null))

(event `CreateWidget`
  (bind _returnvalue (`|CreateWidget` "/Game/UI/WB_TalkingZone.WB_TalkingZone_C"))
  (`UserWidget.AddToViewport` _returnvalue 0)
  (`/Game/UI/WB_TalkingZone.SetText` _returnvalue (`self.Text`))
  (`/Game/UI/WB_TalkingZone.DestoryAfterTime` _returnvalue (`self.DestroyDelay`)))

(fn `UserConstructionScript`
  (`parent.UserConstructionScript`))