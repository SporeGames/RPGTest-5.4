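; Boomerang pickup interactable that unlocks the boomerang on the third-person player character.
; On interaction it plays a 2D pickup sound, sets the character's boomerang flag and switches input from the menu mapping context to the default one.
; If the first quest's first objective is complete it calls the quest; otherwise it replaces that quest with its own and advances a linked NPC's dialogue.
; Both paths destroy the item.
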(event `/Game/Blueprints/InteractionInterface.OnInteraction`
  (params (PlayerCharakter :type "/Game/ThirdPerson/Blueprints/BP_ThirdPersonCharacter Object Reference"))
  (bind _returnvalue (`GameplayStatics.GetPlayerCharacter` 0))
  (bind _quests (`/Game/ThirdPerson/Blueprints/BP_ThirdPersonCharacter.Quests` PlayerCharakter))
  (bind _dialogcomponent (`/Game/Blueprints/NPC/BP_NPC.DialogComponent` (`self.NPCToIncreaseDialog`)))
  (`FMODBlueprintStatics.PlayEvent2D` "/Game/FMOD/Events/CosmeticBekommen.CosmeticBekommen")
  (bind _asbp_third_person_character (cast `/Game/ThirdPerson/Blueprints/BP_ThirdPersonCharacter` _returnvalue))
  (set `/Game/ThirdPerson/Blueprints/BP_ThirdPersonCharacter.BoomerangActiv` true _asbp_third_person_character)
  (message `/Game/Blueprints/BPI_Player.SetPlayerInput` _returnvalue "/Game/ThirdPerson/Input/IMC_Default.IMC_Default" "/Game/ThirdPerson/Input/IMC_Menu.IMC_Menu")
  (if (`/Game/QuestSystem/Objectives/BP_Objective.GetIsComplete` (`|GetArrayItem` (`/Game/QuestSystem/Objectives/BP_ObjCollection.Objectives` (`/Game/QuestSystem/Quests/BP_Quest_Parent.GetRootObjectiveCollection` (`|GetArrayItem` (`/Game/ThirdPerson/Blueprints/BP_ThirdPersonCharacter.Quests` PlayerCharakter))))))
    (`self.CallQuest`)
    (`self.K2_DestroyActor`)
    (else
      (`KismetArrayLibrary.Array_Remove` _quests)
      (`KismetArrayLibrary.Array_Add` _quests (`self.Quest`))
      (set `/Game/DialogSystem/DialogComponent.IncreaseDialoIndex` true _dialogcomponent)
      (bind _result (`/Engine/EditorBlueprintResources/StandardMacros.IncrementInt` (`/Game/DialogSystem/DialogComponent.DialogTreeCounter` _dialogcomponent))
        (:`  `
          (set `/Game/DialogSystem/DialogComponent.DialogTreeCounter` _result _dialogcomponent)
          (`self.K2_DestroyActor`))))))

(fn `UserConstructionScript`)