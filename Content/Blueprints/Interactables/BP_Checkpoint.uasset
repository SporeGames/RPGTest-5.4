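; BP_Checkpoint is an interactable checkpoint with a glyph stone that bobs continuously through two timelines restarting each other.
; The first interaction plays a player montage, saves the player's location as the checkpoint, calls OnInteracted and briefly bursts the Niagara effect in a new color.
; It also starts a looping timer that drains the player's corruption to zero.
; Later interactions open the checkpoint menu widget with mouse-enabled UI input.
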(event `FloatGlyph`
  (bind _felsglypheoberteil (`self.FelsGlypheOberteil`))
  (bind (_direction _floating) (`Timeline|Floating` :!label _label)
    (:`Update`
      (`SceneComponent.K2_SetRelativeLocation` _felsglypheoberteil _floating false false))
    (:`Finished`
      (bind (_direction_2 _floating_2) (`Timeline|Timeline` :!via `ReverseFromEnd`)
        (:`Update`
          (`SceneComponent.K2_SetRelativeLocation` _felsglypheoberteil _floating_2 false false))
        (:`Finished`
          (goto _label :!via `PlayFromStart`))))))

(event `self.ReceiveBeginPlay`
  (`self.FloatGlyph`)
  (bind _asbp_third_person_character (cast `/Game/ThirdPerson/Blueprints/BP_ThirdPersonCharacter` (`GameplayStatics.GetPlayerCharacter` 0)))
  (set `self.As BP Third Person Character` _asbp_third_person_character))

(event `/Game/Blueprints/InteractionInterface.OnInteraction`
  (params (PlayerCharakter :type "/Game/ThirdPerson/Blueprints/BP_ThirdPersonCharacter Object Reference"))
  (bind _returnvalue (`GameplayStatics.GetPlayerController` 0))
  (bind _ns_checkpoint (`self.NS_Checkpoint`))
  (bind _ns_checkpoint_2 (`self.NS_Checkpoint`))
  (if (`self.Interacted`)
    (`|CreateWidget` "/Game/UI/WB_MapSwap.WB_MapSwap_C")
    (`self.HIDEHINT`)
    (bind _returnvalue_2 (`|CreateWidget` "/Game/UI/WB_CheckpintInteractions.WB_CheckpintInteractions_C"))
    (bind _output_get (set `self.Interact` _returnvalue_2))
    (`UserWidget.AddToViewport` _output_get 0)
    (`WidgetBlueprintLibrary.SetInputMode_GameAndUIEx` _returnvalue (`self.Interact`) "LockOnCapture" false)
    (set `PlayerController.bShowMouseCursor` true _returnvalue)
    (else
      (`KismetSystemLibrary.K2_SetTimerDelegate` (delegate `Montage`) 0.001)
      (set `self.Interacted` true)
      (`self.HIDEHINT`)
      (bind _returnvalue_3 (`KismetSystemLibrary.K2_SetTimerDelegate` (delegate `Remove Corruption`) 0.05 true))
      (set `self.RemoveCorruptionTimerOnRespawn` _returnvalue_3)
      (`/Engine/EditorBlueprintResources/StandardMacros.DoOnce` false
        (:`Completed`
          (`FXSystemComponent.SetColorParameter` (`self.NS_Checkpoint`) "ParticleColor" (struct :`R` 52.083351 :`G` 199.999924 :`B` 200.0 :`A` 1.0))
          (`NiagaraComponent.SetNiagaraVariableFloat` _ns_checkpoint_2 "VelocityMaxSpeed" 1500.0)
          (`NiagaraComponent.SetNiagaraVariableFloat` _ns_checkpoint_2 "VelocityMinSpeed" 500.0)
          (`NiagaraComponent.SetNiagaraVariableFloat` _ns_checkpoint_2 "SpawnRate" 250.0)
          (`KismetSystemLibrary.Delay` 1.0)
          (`NiagaraComponent.SetNiagaraVariableFloat` _ns_checkpoint "VelocityMaxSpeed" 100.0)
          (`NiagaraComponent.SetNiagaraVariableFloat` _ns_checkpoint "VelocityMinSpeed" 50.0)
          (`NiagaraComponent.SetNiagaraVariableFloat` _ns_checkpoint "SpawnRate" 10.0))))))

(event `Remove Corruption`
  (`/Game/ThirdPerson/Blueprints/BP_ThirdPersonCharacter.CORRUPT` (`self.As BP Third Person Character`) -20.0)
  (bind _currentcorruption (message `/Game/Blueprints/BPI_Player.GetCurrentCorruption` (`GameplayStatics.GetPlayerCharacter` 0)))
  (if (<= _currentcorruption 0.0)
    (`KismetSystemLibrary.K2_ClearAndInvalidateTimerHandle` (`self.RemoveCorruptionTimerOnRespawn`))))

(event `Montage`
  (`CharacterMovementComponent.SetMovementMode` (`Character.CharacterMovement` (`GameplayStatics.GetPlayerCharacter` 0)) "MOVE_Walking" 0)
  ;[0.1386 1 0.1099] New Anim
  (`|PlayMontage` (`Character.Mesh` (`GameplayStatics.GetPlayerCharacter` 0)) "/Game/Characters/RPG_Character/Animations/SwordAttacks/Attack3_Montage.Attack3_Montage"
    (:`then`
      (set `self.CheckpointLocation` (`self.K2_GetActorLocation` (`GameplayStatics.GetPlayerCharacter` 0)))
      (bind _asbp_third_person_character (cast `/Game/ThirdPerson/Blueprints/BP_ThirdPersonCharacter` (`GameplayStatics.GetPlayerCharacter` 0)))
      (set `/Game/ThirdPerson/Blueprints/BP_ThirdPersonCharacter.CheckPointLocation` (`self.CheckpointLocation`) _asbp_third_person_character)
      (`self.OnInteracted`))))

(event `HIDEHINT`
  (bind _asbp_interaction_hint (cast `/Game/Blueprints/Interactables/BP_InteractionHint` (`ChildActorComponent.ChildActor` (`self.BP_InteractionHint`))))
  (`/Game/Blueprints/Interactables/BP_InteractionHint.HideUIHint` _asbp_interaction_hint))

(fn `UserConstructionScript`)