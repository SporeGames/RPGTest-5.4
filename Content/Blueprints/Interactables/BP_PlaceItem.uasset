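; BP_PlaceItem is an interactable spot where the player places a carried item, or a key item that notifies a Door in the QuestGangolf variant.
; OnInteraction checks the matching player item flag, then reveals the mesh and removes the hint, with montage, sound and cosmetic detach for regular items.
; Without the item, a timed self-talk widget appears, skipped in the regular branch if another is alive.
; The construction script picks the cosmetic to detach.
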(event `/Game/Blueprints/InteractionInterface.OnInteraction`
  (params (PlayerCharakter :type "/Game/ThirdPerson/Blueprints/BP_ThirdPersonCharacter Object Reference"))
  (bind _output_get (set `self.Player Charakter` PlayerCharakter))
  (if (`self.QuestGangolf`)
    (if (`/Game/ThirdPerson/Blueprints/BP_ThirdPersonCharacter.ItemKeyActive` (`self.Player Charakter`))
      (`StaticMeshComponent.SetStaticMesh` (`self.Sphere`) (`self.New Mesh`))
      (`SceneComponent.SetVisibility` (`self.Sphere`) true false)
      (`ActorComponent.K2_DestroyComponent` (`self.BP_InteractionHint`))
      (set `PrimitiveComponent.bGenerateOverlapEvents` false (`self.Sphere`))
      (`/Game/Blueprints/Interactables/BP_Door.ItemPlaced` (`self.Door`))
      (`/Game/ThirdPerson/Blueprints/BP_ThirdPersonCharacter.SetPlayerInput` (`self.Player Charakter`) "/Game/ThirdPerson/Input/IMC_Default.IMC_Default" "/Game/ThirdPerson/Input/IMC_Menu.IMC_Menu")
      (else
        (`self.SelfTalk`)))
    (elif (select `int` (`self.ItemIndex`) :`0` (`/Game/ThirdPerson/Blueprints/BP_ThirdPersonCharacter.ItemActive` _output_get) :`1` (`/Game/ThirdPerson/Blueprints/BP_ThirdPersonCharacter.ItemActive2` _output_get) :`2` (`/Game/ThirdPerson/Blueprints/BP_ThirdPersonCharacter.ItemActive3` _output_get))
      (set `/Game/ThirdPerson/Blueprints/BP_ThirdPersonCharacter.ItemActive` false (`self.Player Charakter`))
      ;[1 1 1] Placing Item
      (`|PlayMontage` null
        (:`then`
          (`StaticMeshComponent.SetStaticMesh` (`self.Sphere`) (`self.New Mesh`))
          (`SceneComponent.SetVisibility` (`self.Sphere`) true false)
          (`/Game/ThirdPerson/Blueprints/BP_ThirdPersonCharacter.SetPlayerInput` (`self.Player Charakter`) "/Game/ThirdPerson/Input/IMC_Default.IMC_Default" "/Game/ThirdPerson/Input/IMC_Menu.IMC_Menu")
          (if (== (`self.ItemIndex`) 1)
            (`SceneComponent.SetWorldScale3D` (`self.Sphere`) (0.1 0.1 0.1)))
          (`ActorComponent.K2_DestroyComponent` (`self.BP_InteractionHint`))
          (set `PrimitiveComponent.bGenerateOverlapEvents` false (`self.Sphere`))
          (`self.OnInteracted`)
          (message `/Game/Blueprints/BPI_Player.DeactivateCosmetic` (`GameplayStatics.GetPlayerCharacter` 0) false (`|MakeArray` (`self.Detach Cosmetic`)))
          (`FMODBlueprintStatics.PlayEvent2D` (`self.PlaceSound`))))
      (else
        (bind _foundwidgets (`WidgetBlueprintLibrary.GetAllWidgetsOfClass` "/Game/UI/WB_TalkingZone.WB_TalkingZone_C"))
        (for _array_element _foundwidgets
          (if (`/Game/UI/WB_TalkingZone.Alive?` _array_element)
            (set `self.TalkingZoneActive` true)))
        (if (`self.TalkingZoneActive`)
          (`/Game/ThirdPerson/Blueprints/BP_ThirdPersonCharacter.SetPlayerInput` (`self.Player Charakter`) "/Game/ThirdPerson/Input/IMC_Default.IMC_Default" "/Game/ThirdPerson/Input/IMC_Menu.IMC_Menu")
          (else
            (`self.SelfTalk`)))))))

(event `SelfTalk`
  (bind _returnvalue (`|CreateWidget` "/Game/UI/WB_TalkingZone.WB_TalkingZone_C"))
  (`UserWidget.AddToViewport` _returnvalue 0)
  (`/Game/UI/WB_TalkingZone.SetText` _returnvalue (`self.SelfTalkText`))
  (`/Game/ThirdPerson/Blueprints/BP_ThirdPersonCharacter.SetPlayerInput` (`self.Player Charakter`) "/Game/ThirdPerson/Input/IMC_Default.IMC_Default" "/Game/ThirdPerson/Input/IMC_Menu.IMC_Menu")
  (`KismetSystemLibrary.Delay` (`self.DeleteSelfTalkAfterTime`))
  (`/Game/UI/WB_TalkingZone.Destroy` _returnvalue)
  (set `self.TalkingZoneActive` false))

(fn `UserConstructionScript`
  (bind _sphere (`self.Sphere`))
  (if (== _sphere "/Game/Art/Enviroment/Kleinkram/Leinwand.Leinwand")
    (set `self.Detach Cosmetic` "/Game/Art/Attachments/DA_Picture.DA_Picture")
    (elif (== _sphere "/Game/Art/EnemySmall/Waffen/Teddy/TeddyMesh.TeddyMesh")
      (set `self.Detach Cosmetic` "/Game/Art/Attachments/DA_Teddy.DA_Teddy")
      (elif true
        _))))