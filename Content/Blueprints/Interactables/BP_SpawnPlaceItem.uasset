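; BP_SpawnPlaceItem is an interactable spawner that places a BP_PlaceItem actor in the level when its SpawnSphere event is called.
; The spawn transform takes its location from the Sphere component and its rotation from the Arrow component.
; It passes its mesh, item index and place sound through, plus a fixed German self-talk line about lacking the right item.
; A delayed self-trigger exists but is unconnected.
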(event `self.ReceiveBeginPlay`)

(event `SpawnSphere`
  (`|SpawnActorFromClass` "/Game/Blueprints/Interactables/BP_PlaceItem.BP_PlaceItem_C" (`KismetMathLibrary.MakeTransform` (`SceneComponent.K2_GetComponentLocation` (`self.Sphere`)) (`SceneComponent.K2_GetComponentRotation` (`self.Arrow`))) "Undefined" "MultiplyWithRoot" null 0.2 "Leider fehlt mir das richtige Item" (`self.New Mesh`) (`self.Item Index`) (`self.Place Sound`) null))

(fn `UserConstructionScript`)