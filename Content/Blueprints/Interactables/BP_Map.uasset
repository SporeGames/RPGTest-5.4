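; Interactable map Blueprint that opens the map swap menu when the player interacts with it.
; OnInteraction pauses the game, sets game-only input, shows the mouse cursor and adds a new WB_MapSwap widget with an empty map name to the viewport.
; A debug key removes the widget and unpauses, setting cursor visibility from SetGamePaused's return value rather than explicitly hiding it.
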(event EventOnInteraction
  (params (PlayerCharakter :type BP%20Third%20Person%20Character%20Object%20Reference))
  (bind _returnvalue (Game|GetPlayerController 0))
  (Game|SetGamePaused true)
  (Input|SetInputModeGameOnly _returnvalue false)
  (Variables|/Script/Engine.PlayerController|SetbShowMouseCursor _returnvalue true)
  (bind _returnvalue_2 (UserInterface|CreateWidget "/Game/UI/WB_MapSwap.WB_MapSwap_C"))
  (bind _output_get (Variables|Default|SetMap _returnvalue_2))
  (UserInterface|Viewport|AddtoViewport _output_get 0))

(event Input|KeyboardEvents|DebugKey6
  (params (Key :type Key%20Structure :default "None") (ActionValue :type Input%20Action%20Value%20Structure))
  (:Pressed
    (Widget|RemovefromParent (Variables|Default|GetMap))
    (bind _returnvalue (Game|SetGamePaused false))
    (Variables|/Script/Engine.PlayerController|SetbShowMouseCursor (Game|GetPlayerController 0) _returnvalue)))

(event Input|KeyboardEvents|Escape
  (params (Key :type Key%20Structure :default "None")))

(fn ConstructionScript)