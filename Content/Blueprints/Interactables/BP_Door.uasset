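; Puzzle door that opens once via a button, or when its linked pressure plates, targets and optional item placement are satisfied.
; Plate and target events count active elements and cross-check each other; item placement opens it only if all targets are already flagged active and the plate count matches.
; Opening plays sound events, then timelines either slide both halves apart and destroy them, or lower them at a GoDownTime-based rate.
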(event `self.ReceiveBeginPlay`
  (set `self.NumberOfPressurePlates` (`KismetArrayLibrary.Array_Length` (`self.PressurePlates`)))
  (set `self.NumberOfTargets` (`KismetArrayLibrary.Array_Length` (`self.Targets`))))

(event `/Game/Blueprints/Interactables/BPI_Button.OnButtonPressed`
  (params (Button :type "/Game/Blueprints/Interactables/BP_Button Object Reference"))
  (`self.OpenDoor`))

(event `OpenDoor`
  (bind _returnvalue (`self.K2_GetActorLocation`))
  (`/Engine/EditorBlueprintResources/StandardMacros.DoOnce` false
    (:`Completed`
      (`FMODBlueprintStatics.PlayEventAtLocation` "/Game/FMOD/Events/Tür.Tür" (`KismetMathLibrary.MakeTransform` _returnvalue))
      (`FMODBlueprintStatics.PlayEventAtLocation` (`self.MechanismusSound`) (`KismetMathLibrary.MakeTransform` _returnvalue))
      (if (not (`self.Down?`))
        (bind (_direction _down) (`Timeline|Open Door` :!via `PlayFromStart`)
          (:`Update`
            (`SceneComponent.K2_AddRelativeLocation` (`self.Cube_R`) (`KismetMathLibrary.MakeVector` (`KismetMathLibrary.Lerp` 0.0 5.0 _down)) false false)
            (`SceneComponent.K2_AddRelativeLocation` (`self.Cube_L`) (`KismetMathLibrary.MakeVector` (`KismetMathLibrary.Lerp` 0.0 -5.0 _down)) false false))
          (:`Finished`
            (`ActorComponent.K2_DestroyComponent` (`self.Cube_L`))
            (`ActorComponent.K2_DestroyComponent` (`self.Cube_R`))))
        (else
          (`TimelineComponent.SetPlayRate` (`self.Door Down`) (/ 1.0 (`self.Go Down Time`)))
          (bind (_direction_2 _alpha) (`Timeline|Door Down` :!via `PlayFromStart`)
            (:`Update`
              (bind _returnvalue_2 (`KismetMathLibrary.Lerp` 0.0 -150.0 _alpha))
              (`SceneComponent.K2_AddRelativeLocation` (`self.Cube_R`) (`KismetMathLibrary.MakeVector` 0.0 0.0 _returnvalue_2) false false)
              (`SceneComponent.K2_AddRelativeLocation` (`self.Cube_L`) (`KismetMathLibrary.MakeVector` 0.0 0.0 _returnvalue_2) false false))))))))

(event `/Game/Blueprints/Interactables/BPI_Button.PressurePlateActive`
  (for _array_element (`self.PressurePlates`)
    (if (`/Game/Blueprints/Interactables/BP_PressurePlate.Active` _array_element)
      (`/Engine/EditorBlueprintResources/StandardMacros.IncrementInt` (`self.CounterPressurePlates`))))
  (if (== (`self.CounterPressurePlates`) (`self.NumberOfPressurePlates`))
    (if (`KismetArrayLibrary.Array_IsEmpty` (`self.Targets`))
      (if (`self.ItemPlaced?`)
        (`self.OpenDoor` :!label _label)
        (elif (not (`KismetSystemLibrary.IsValid` (`self.PlaceItem`)))
          (goto _label)))
      (elif (`self.AllTargetActiv`)
        (if (`self.ItemPlaced?`)
          (`self.OpenDoor` :!label _label_2)
          (elif (not (`KismetSystemLibrary.IsValid` (`self.PlaceItem`)))
            (goto _label_2)))
        (else
          (set `self.CounterPressurePlates` 0))))
    (else
      (set `self.CounterPressurePlates` 0))))

(event `/Game/Blueprints/Interactables/BPI_Button.TargetActive`
  (for _array_element (`self.Targets`)
    (if (`/Game/Blueprints/Interactables/BP_Target.Active` _array_element)
      (`/Engine/EditorBlueprintResources/StandardMacros.IncrementInt` (`self.CounterTargets`))))
  (if (== (`self.CounterTargets`) (`self.NumberOfTargets`))
    (set `self.AllTargetActiv` true)
    (if (`KismetArrayLibrary.Array_IsEmpty` (`self.PressurePlates`))
      (if (`self.ItemPlaced?`)
        (`self.OpenDoor` :!label _label_3)
        (elif (not (`KismetSystemLibrary.IsValid` (`self.PlaceItem`)))
          (goto _label_3)))
      (else
        (set `self.CounterPressurePlates` 0)
        (for _array_element_2 (`self.PressurePlates`)
          (if (`/Game/Blueprints/Interactables/BP_PressurePlate.Active` _array_element_2)
            (`/Engine/EditorBlueprintResources/StandardMacros.IncrementInt` (`self.CounterPressurePlates`))))
        (if (== (`self.CounterPressurePlates`) (`self.NumberOfPressurePlates`))
          (if (`self.ItemPlaced?`)
            (`self.OpenDoor` :!label _label_4)
            (elif (not (`KismetSystemLibrary.IsValid` (`self.PlaceItem`)))
              (goto _label_4)))
          (else
            (set `self.CounterPressurePlates` 0)))))
    (else
      (set `self.CounterTargets` 0))))

(event `/Game/Blueprints/Interactables/BPI_Button.ItemPlaced`
  (set `self.ItemPlaced?` true)
  (if (`self.AllTargetActiv`)
    (if true
      (if (== (`self.CounterPressurePlates`) (`self.NumberOfPressurePlates`))
        (`self.OpenDoor`)))))

(fn `UserConstructionScript`)