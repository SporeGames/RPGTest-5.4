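; BP_Button is an interactable button that notifies a set of linked objects when the player interacts with it.
; At BeginPlay it casts ObjectsToInteractWith to BPI_Button and caches them uniquely in NewVar.
; On interaction it sets the player character's movement mode to Walking, then calls OnButtonPressed on each cached object, passing itself.
; Within that loop it also hides the UI hint of its BP_InteractionHint child actor.
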(event `self.ReceiveBeginPlay`
  (for _array_element (`self.ObjectsToInteractWith`)
    (bind _asbpi_button (cast `/Game/Blueprints/Interactables/BPI_Button` _array_element))
    (`KismetArrayLibrary.Array_AddUnique` (`self.NewVar`) _asbpi_button)))

(event `/Game/Blueprints/InteractionInterface.OnInteraction`
  (params (PlayerCharakter :type "/Game/ThirdPerson/Blueprints/BP_ThirdPersonCharacter Object Reference"))
  (`CharacterMovementComponent.SetMovementMode` (`Character.CharacterMovement` (`GameplayStatics.GetPlayerCharacter` 0)) "MOVE_Walking" 0)
  (for _array_element (`self.NewVar`)
    (`/Game/Blueprints/Interactables/BPI_Button.OnButtonPressed` _array_element self)
    (bind _asbp_interaction_hint (cast `/Game/Blueprints/Interactables/BP_InteractionHint` (`ChildActorComponent.ChildActor` (`self.BP_InteractionHint`)))
      (:`then`
        (`/Game/Blueprints/Interactables/BP_InteractionHint.HideUIHint` _asbp_interaction_hint))
      (:`CastFailed`
        (`KismetSystemLibrary.PrintString` "failed :(")))))

(fn `UserConstructionScript`)