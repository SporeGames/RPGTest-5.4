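; BP_Glyph is an interactable pickup that the player collects to raise a glyph counter on BP_ThirdPersonCharacter.
; On interaction it casts the player character, increments its GlpyhCount and prints the new total to screen.
; The count then selects one of three tiers for the character's Saeckengroesse (sack size) enum.
; The glyph destroys itself afterwards.
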(event `self.ReceiveBeginPlay`)

(event `self.OnInteraction`
  (params (PlayerCharakter :type "/Game/ThirdPerson/Blueprints/BP_ThirdPersonCharacter Object Reference"))
  (bind _asbp_third_person_character (cast `/Game/ThirdPerson/Blueprints/BP_ThirdPersonCharacter` (`GameplayStatics.GetPlayerCharacter` 0)))
  (bind _glpyhcount (`/Game/ThirdPerson/Blueprints/BP_ThirdPersonCharacter.GlpyhCount` _asbp_third_person_character))
  (bind _result (`/Engine/EditorBlueprintResources/StandardMacros.IncrementInt` _glpyhcount)
    (:`  `
      (`KismetSystemLibrary.PrintString` (`KismetStringLibrary.Conv_IntToString` _glpyhcount))
      (if (<= _glpyhcount 3)
        (set `/Game/ThirdPerson/Blueprints/BP_ThirdPersonCharacter.Saeckengroesse` "NewEnumerator0" _asbp_third_person_character)
        (elif (<= _result 6)
          (set `/Game/ThirdPerson/Blueprints/BP_ThirdPersonCharacter.Saeckengroesse` "NewEnumerator1" _asbp_third_person_character)
          (else
            (set `/Game/ThirdPerson/Blueprints/BP_ThirdPersonCharacter.Saeckengroesse` "NewEnumerator2" _asbp_third_person_character))))
      (`self.K2_DestroyActor`))))

(fn `UserConstructionScript`)