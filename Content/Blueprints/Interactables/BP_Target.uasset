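; BP_Target is an interactable target that activates when a boomerang hits it and notifies a linked door.
; A sphere overlap checks the other actor for the Boomerang tag, then triggers activation and hit feedback.
; Activation plays a mechanism sound at the target's location, sets the Active flag and calls TargetActiveMessage on the Door reference.
; Hit feedback swaps the material on the target mesh.
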(event `self.Sphere.OnComponentBeginOverlap`
  (params (OverlappedComponent :type "PrimitiveComponent Object Reference") (OtherActor :type "Actor Object Reference") (OtherComp :type "PrimitiveComponent Object Reference") (OtherBodyIndex :type Integer) (bFromSweep :type Boolean) (SweepResult :type "HitResult Structure (by ref)"))
  (if (`self.ActorHasTag` OtherActor "Boomerang")
    (`KismetSystemLibrary.PrintString` "Boomerang")
    (`self.ActivateEvent`)
    (`self.HitFeedback`)))

(event `ActivateEvent`
  (`FMODBlueprintStatics.PlayEventAtLocation` "/Game/FMOD/Events/Mechanismus_Activated.Mechanismus_Activated" (`KismetMathLibrary.MakeTransform` (`self.K2_GetActorLocation`)))
  (set `self.Active` true)
  (message `/Game/Blueprints/Interactables/BPI_Button.TargetActive` (`self.Door`)))

(event `HitFeedback`
  (`PrimitiveComponent.SetMaterial` (`self.Target`) 0 "/Game/Art/Enviroment/Gebäude/Heimathaus/HausGeländer_Material.HausGeländer_Material"))

(fn `UserConstructionScript`)