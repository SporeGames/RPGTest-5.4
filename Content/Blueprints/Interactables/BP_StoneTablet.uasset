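; BP_StoneTablet is an interactable that shows a stone tablet image to the player in a UI widget.
; On interaction it disables player movement, creates a WB_StoneTablet widget and switches to UI-only input with the mouse cursor visible.
; The widget's image is set from the StoneTabletTexture variable at native size; this Blueprint itself does not restore movement or input.
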(event `/Game/Blueprints/InteractionInterface.OnInteraction`
  (params (PlayerCharakter :type "/Game/ThirdPerson/Blueprints/BP_ThirdPersonCharacter Object Reference"))
  (bind _returnvalue (`GameplayStatics.GetPlayerController` 0))
  (`CharacterMovementComponent.DisableMovement` (`Character.CharacterMovement` (`GameplayStatics.GetPlayerCharacter` 0)))
  (bind _returnvalue_2 (`|CreateWidget` "/Game/UI/WB_StoneTablet.WB_StoneTablet_C" (`GameplayStatics.GetPlayerController` 0)))
  (`UserWidget.AddToViewport` _returnvalue_2 0)
  (`WidgetBlueprintLibrary.SetInputMode_UIOnlyEx` _returnvalue _returnvalue_2)
  (set `PlayerController.bShowMouseCursor` true _returnvalue)
  (`Image.SetBrushFromTexture` (`/Game/UI/WB_StoneTablet.StoneTabletImage` _returnvalue_2) (`self.StoneTabletTexture`) true)
  (set `self.Key` (struct)))

(fn `UserConstructionScript`)