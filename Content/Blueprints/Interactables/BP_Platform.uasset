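; Interactable platform that breaks away shortly after an actor tagged Player overlaps its Box.
; The overlap immediately spawns and triggers an FS_MasterField at the actor's location, then after a delay spawns BP_DestructablePlatformSpawn at the Platform's position.
; A brief second delay precedes destroying the Platform component, so the destructible stand-in replaces it.
; An alternative physics-and-gravity drop is left unconnected and never runs.
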(event `self.ReceiveBeginPlay`)

(event `self.HitByPhysic`
  (params (`Hit Location` :type "Vector Structure")))

(event `self.Box.OnComponentBeginOverlap`
  (params (OverlappedComponent :type "PrimitiveComponent Object Reference") (OtherActor :type "Actor Object Reference") (OtherComp :type "PrimitiveComponent Object Reference") (OtherBodyIndex :type Integer) (bFromSweep :type Boolean) (SweepResult :type "HitResult Structure (by ref)"))
  (bind _platform (`self.Platform`))
  (bind _returnvalue_location (`KismetMathLibrary.BreakTransform` (`SceneComponent.K2_GetComponentToWorld` _platform)))
  (if (`self.ActorHasTag` OtherActor "Player")
    (bind _returnvalue (`|SpawnActorFromClass` "/Engine/EditorResources/FieldNodes/FS_MasterField.FS_MasterField_C" (`KismetMathLibrary.MakeTransform` (`self.K2_GetActorLocation`)) "Undefined" "MultiplyWithRoot" null null))
    (set `/Engine/EditorResources/FieldNodes/FS_MasterField.ActivationType` "NewEnumerator4" _returnvalue)
    (`/Engine/EditorResources/FieldNodes/FS_MasterField.CE_Trigger` _returnvalue)
    (bind _output_get (set `self.Location` _returnvalue_location))
    (`KismetSystemLibrary.Delay` 1.5)
    (`|SpawnActorFromClass` "/Game/Blueprints/Interactables/BP_DestructablePlatformSpawn.BP_DestructablePlatformSpawn_C" (`KismetMathLibrary.MakeTransform` _output_get) "Undefined" "MultiplyWithRoot" null null)
    (`KismetSystemLibrary.Delay` 0.2)
    (`ActorComponent.K2_DestroyComponent` _platform)))

(fn `UserConstructionScript`)