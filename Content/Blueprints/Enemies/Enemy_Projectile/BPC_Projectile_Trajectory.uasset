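; Enemy projectile trajectory component that builds an arced spline path from an actor to a goal location.
; CalculateSpline turns the actor and spline toward the goal, then places evenly spaced points along that line.
; Each point's Z offset is a runtime curve value scaled by distance travelled, with an extra point dipping just past the goal.
; Spline duration scales with point count and is returned to the caller.
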(fn `Calculate Spline`
  (params (`Actor location` :type "Actor Object Reference") (Spline :type "SplineComponent Object Reference") (`Goal Location` :type "Vector Structure") (Abstand :type "Float (double-precision)"))
  (returns (Duration :type "Float (double-precision)"))
  (bind _returnvalue (`KismetMathLibrary.FindLookAtRotation` (`self.Origin Point`) (`self.Goal Location`)))
  (bind (_returnvalue_x _returnvalue_y _returnvalue_z) (`KismetMathLibrary.BreakVector` (+ (`self.Origin Point`) (* (* (+ (`self.Number of Points`) 1) (`self.Abstand`)) (`Actor.GetActorForwardVector` `Actor location`)))))
  (set `self.Spline` Spline)
  (set `self.Goal Location` `Goal Location`)
  (set `self.Origin Point` (`Actor.K2_GetActorLocation` `Actor location`))
  (set `self.Abstand` Abstand)
  (set `self.Number of Points` (`KismetMathLibrary.Round` (/ (`KismetMathLibrary.Abs` (`KismetMathLibrary.Vector_Distance` (`self.Origin Point`) (`self.Goal Location`))) (`self.Abstand`))))
  (`SceneComponent.K2_SetWorldRotation` (`self.Spline`) _returnvalue false false)
  (`Actor.K2_SetActorRotation` `Actor location` _returnvalue true)
  (set `self.Unit Direction` (- (`self.Origin Point`) (`self.Goal Location`)))
  (set `self.Curve Time Intervall` (/ 1.0 (`KismetMathLibrary.Conv_IntToDouble` (`self.Number of Points`))))
  (set `self.Duration` (* (`self.Number of Points`) (`self.Duration Ratio`)))
  (for _index (range (+ (`self.Number of Points`) 1))
    (set `self.Height` (`KismetMathLibrary.GetRuntimeFloatCurveValue` (`self.Curve`) (* _index (`self.Curve Time Intervall`))))
    (bind (_returnvalue_x_2 _returnvalue_y_2 _returnvalue_z_2) (`KismetMathLibrary.BreakVector` (+ (`self.Origin Point`) (* (* _index (`self.Abstand`)) (`Actor.GetActorForwardVector` `Actor location`)))))
    (bind _returnvalue_2 (+ _returnvalue_z_2 (* (* (`self.Abstand`) _index) (`self.Height`))))
    (`KismetSystemLibrary.SphereTraceSingle` :`Start` (`KismetMathLibrary.MakeVector` _returnvalue_x_2 _returnvalue_y_2 _returnvalue_2) :`End` (`KismetMathLibrary.MakeVector` _returnvalue_x_2 _returnvalue_y_2 _returnvalue_2) :`Radius` 30.0 :`TraceChannel` "TraceTypeQuery1" :`DrawDebugType` "ForDuration" :`DrawTime` 1.0 :!enabledstate Disabled)
    (`KismetArrayLibrary.Array_Add` (`self.All Points`) (`KismetMathLibrary.MakeVector` _returnvalue_x_2 _returnvalue_y_2 _returnvalue_2))
    (if (== _index (`self.Number of Points`))
      (`KismetArrayLibrary.Array_Add` (`self.All Points`) (`KismetMathLibrary.MakeVector` _returnvalue_x _returnvalue_y (+ _returnvalue_z (* (* (`self.Abstand`) (+ (`self.Number of Points`) 1)) -0.15))))))
  (`SplineComponent.SetSplinePoints` (`self.Spline`) (`self.All Points`) "World" true)
  (bind _output_get (set `SplineComponent.Duration` (`self.Duration`) (`self.Spline`)))
  (return _output_get))