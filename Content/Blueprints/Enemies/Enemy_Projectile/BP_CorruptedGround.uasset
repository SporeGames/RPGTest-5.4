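; BP_CorruptedGround is an enemy ground hazard that repeatedly damages players standing inside its sphere.
; A looping half-second timer started on BeginPlay polls the sphere's overlapping actors and sends each Player-tagged one a TakeDMGMessage with hit reaction and a damage type.
; The sphere's begin-overlap event only prints the player's overlapping component name for debugging, and each damage tick also prints a debug string.
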(event `self.ReceiveBeginPlay`
  (`KismetSystemLibrary.K2_SetTimerDelegate` (delegate `Deal Damage`) 0.5 true))

(event `Deal Damage`
  (for _array_element (`PrimitiveComponent.GetOverlappingActors` (`self.Sphere`) null)
    (if (`self.ActorHasTag` _array_element "Player")
      (`KismetSystemLibrary.PrintString` "GROUND CORRUPT" true true (struct :`R` 0.994216 :`G` 1.0 :`B` 0.510306 :`A` 1.0) 2.0 "fesgf")
      (message `/Game/Blueprints/Enemies/BPI_Damagable.Take DMG` _array_element 2.0 true "NewEnumerator4"))))

(event `self.Sphere.OnComponentBeginOverlap`
  (params (OverlappedComponent :type "PrimitiveComponent Object Reference") (OtherActor :type "Actor Object Reference") (OtherComp :type "PrimitiveComponent Object Reference") (OtherBodyIndex :type Integer) (bFromSweep :type Boolean) (SweepResult :type "HitResult Structure (by ref)"))
  (if (`self.ActorHasTag` OtherActor "Player")
    (`KismetSystemLibrary.PrintString` (`KismetSystemLibrary.GetDisplayName` OtherComp) true true (struct :`R` 1.0 :`G` 0.949031 :`B` 0.485349 :`A` 1.0) 2.0 "htfdh")))

(fn `UserConstructionScript`)