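; Enemy ranged projectile that flies along a spline trajectory and explodes on impact to damage the player.
; Shoot has BPCProjectileTrajectory build the spline, then a looping timer sweeps the projectile along it by time until the returned value is exceeded and the actor is destroyed.
; On hit it stops the timer, plays a sound, applies damage through a debug-drawn sphere trace, then destroys itself after a short delay.
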(event `Shoot`
  (params (`Target Location` :type "Vector Structure") (Instigator :type "Actor Object Reference") (Abstand :type "Float (double-precision)"))
  (bind _duration (`/Game/Blueprints/Enemies/Enemy_Projectile/BPC_Projectile_Trajectory.Calculate Spline` (`self.BPC_Projectile_Trajectory`) self (`self.Spline`) `Target Location` Abstand))
  (bind _returnvalue (`KismetSystemLibrary.K2_SetTimerDelegate` (delegate `Move Arrow`) 0.001 true)))

(event `Move Arrow`
  (bind _output_get (set `self.Active Time` (+ (`self.Active Time`) 0.001)))
  (bind (_returnvalue_location _returnvalue_rotation) (`KismetMathLibrary.BreakTransform` (`SplineComponent.GetTransformAtTime` (`self.Spline`) _output_get "World" false false)))
  (`SceneComponent.K2_SetWorldLocationAndRotation` (`self.Projectile`) _returnvalue_location _returnvalue_rotation true false)
  (if (> (`self.Active Time`) (stale `Shoot` _duration))
    (`KismetSystemLibrary.K2_ClearAndInvalidateTimerHandle` (stale `Shoot` _returnvalue))
    (`self.K2_DestroyActor`)))

(event `self.Projectile.OnComponentHit`
  (params (HitComponent :type "PrimitiveComponent Object Reference") (OtherActor :type "Actor Object Reference") (OtherComp :type "PrimitiveComponent Object Reference") (NormalImpulse :type "Vector Structure") (Hit :type "HitResult Structure (by ref)"))
  (bind _returnvalue (`GameplayStatics.GetPlayerCharacter` 0))
  (`|ExecutionSequence`
    (:`then_0`
      (`KismetSystemLibrary.K2_ClearAndInvalidateTimerHandle` (stale `Shoot` _returnvalue)))
    (:`then_1`
      ;[1 1 1] KIM Environment Hit Sound - Explosion sound, idk
      (`GameplayStatics.PlaySoundAtLocation` null Hit_ImpactPoint (struct) 1.0 1.0 0.0 null null null null)
      (bind _outhits (`KismetSystemLibrary.SphereTraceMulti` :`Start` Hit_ImpactPoint :`End` Hit_ImpactPoint :`Radius` (`self.Explosion Radius`) :`TraceChannel` "TraceTypeQuery1" :`DrawDebugType` "ForDuration" :`DrawTime` 2.0))
      (for _array_element _outhits
        (bind (_bblockinghit _binitialoverlap _time _distance _location _impactpoint _normal _impactnormal _physmat _hitactor) (`GameplayStatics.BreakHitResult` _array_element))
        (if (== _hitactor _returnvalue)
          (message `/Game/Blueprints/Enemies/BPI_Damagable.Take DMG` _returnvalue 5.0)))
      (`KismetSystemLibrary.Delay` 0.2)
      (`KismetSystemLibrary.PrintString` (`KismetSystemLibrary.GetDisplayName` _hitactor))
      (`self.K2_DestroyActor`))))

(fn `UserConstructionScript`)