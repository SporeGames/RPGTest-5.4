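; Ranged enemy, a child of a parent enemy class, that throws projectiles at the player.
; Attack index 0 plays a throw montage whose notify spawns a projectile at ThrowPoint, aimed at the player's position; completion signals attack finished.
; Death plays a montage, halts movement and AI logic, then destroys the actor on a notify.
; The parent death event also triggers a one-time Niagara aura and timeline-driven dissolve on a dynamic material.
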(event `self.ReceiveBeginPlay`
  (`parent.ReceiveBeginPlay`)
  (bind _returnvalue (`PrimitiveComponent.CreateDynamicMaterialInstance` (`self.Mesh`) 0 "/Game/Art/EnemySmall/M_Dissolve_Inst.M_Dissolve_Inst" "None"))
  (bind _output_get (set `self.BigBody` _returnvalue))
  (`MaterialInstanceDynamic.SetVectorParameterValue` _output_get "DissolveColor" (`self.Value`))
  (add `self.Death` (delegate `onDeath`)))

(event `onDeath`
  (bind _notifyname (`|PlayMontage` (`self.Mesh`) "/Game/Art/EnemyBig/Animation/BigEnemyDie_Montage.BigEnemyDie_Montage")
    (:`then`
      (set `CharacterMovementComponent.MaxWalkSpeed` 0.0 (`self.CharacterMovement`))
      (`BrainComponent.StopLogic` (`AIController.BrainComponent` (`AIBlueprintHelperLibrary.GetAIController` self)) ""))
    (:`OnNotifyBegin`
      (switch `name` _notifyname
        (:`dead`
          (`self.K2_DestroyActor`))))))

(event `/Game/Blueprints/Enemies/BPI_Enemy.Attack Index`
  (params (`Attack Index` :type Integer))
  (bind _returnvalue_location (`KismetMathLibrary.BreakTransform` (`SceneComponent.K2_GetComponentToWorld` (`self.ThrowPoint`))))
  (switch `int` `Attack Index`
    (:`Default`
      (`KismetSystemLibrary.PrintString` "NO VALID ATTACK INDEX"))
    (:`0`
      (bind _notifyname (`|PlayMontage` (`self.Mesh`) "/Game/Art/EnemyBig/Animation/BigEnemyThrow_Montage.BigEnemyThrow_Montage" 0.7)
        (:`OnCompleted`
          (`self.AttackFinished`))
        (:`OnNotifyBegin`
          (switch `name` _notifyname
            (:`Throw`
              (bind _returnvalue (`|SpawnActorFromClass` "/Game/Blueprints/Enemies/Enemy_Projectile/BP_Enemy_Ranged_Projectile.BP_Enemy_Ranged_Projectile_C" (`KismetMathLibrary.MakeTransform` _returnvalue_location) "AlwaysSpawn" "MultiplyWithRoot" null null))
              (`/Game/Blueprints/Enemies/Enemy_Projectile/BP_Enemy_Ranged_Projectile.Shoot` _returnvalue (`self.K2_GetActorLocation` (`GameplayStatics.GetPlayerCharacter` 0)) self 100.0))))))))

(event `self.Death Parent`
  (bind _bigbody (`self.BigBody`))
  (`parent.Death Parent`)
  (`/Engine/EditorBlueprintResources/StandardMacros.DoOnce` false
    (:`Completed`
      (`NiagaraFunctionLibrary.SpawnSystemAttached` "/Game/Art/Particle/DashTrail/NS_AuraSmall.NS_AuraSmall" (`self.Mesh`) "None" (0.0 0.0 0.0) (struct) "KeepRelativeOffset")
      (bind (_direction _dissolve _smoothnes) (`Timeline|Timeline`)
        (:`Update`
          (`MaterialInstanceDynamic.SetScalarParameterValue` _bigbody "Dissolve" _dissolve)
          (`MaterialInstanceDynamic.SetScalarParameterValue` _bigbody "TransitionSmoothness" _smoothnes))))))

(fn `UserConstructionScript`
  (`parent.UserConstructionScript`))