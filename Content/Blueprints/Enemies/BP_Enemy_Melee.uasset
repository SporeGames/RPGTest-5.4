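; Melee enemy Blueprint that gives its idle weapon a random wrench, shovel or pitchfork mesh on BeginPlay.
; Attack index 0 swaps the idle weapon for the combat weapon, plays a hit montage, then restores visibility and signals attack finished on completion.
; Weapon trace events start and stop the sword trace in BPCAttackSystem, and GetWeaponTrace supplies the combat weapon's Top and Bottom socket locations.
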(event `self.ReceiveBeginPlay`
  (`parent.ReceiveBeginPlay`)
  (`StaticMeshComponent.SetStaticMesh` (`self.Weapon_Idle`) (select `int` (`KismetMathLibrary.RandomIntegerInRange` 0 2) :`0` "/Game/Art/EnemySmall/Waffen/Schraubenschlüssel.Schraubenschlüssel" :`1` "/Game/Art/EnemySmall/Waffen/Schaufel.Schaufel" :`2` "/Game/Art/EnemySmall/Waffen/Mistgabel.Mistgabel" :!type "StaticMesh Object Reference")))

(event `/Game/Blueprints/Enemies/BPI_Enemy.Attack Index`
  (params (`Attack Index` :type Integer))
  (switch `int` `Attack Index`
    (:`Default`
      (`KismetSystemLibrary.PrintString` "NO VALID ATTACK INDEX"))
    (:`0`
      (`self.Set Weapon Visibility` (`self.Weapon_Combat`))
      (`self.Set Weapon Visibility` (`self.Weapon_Idle`) true)
      (`|PlayMontage` (`self.Mesh`) "/Game/Art/EnemySmall/Animationen/SmallEnemyHit_Montage.SmallEnemyHit_Montage"
        (:`OnCompleted`
          (`self.AttackFinished`))
        (:`OnBlendOut`
          _))
      (`self.Set Weapon Visibility` (`self.Weapon_Combat`) true)
      (`self.Set Weapon Visibility` (`self.Weapon_Idle`)))))

(event `/Game/Blueprints/Enemies/BPI_Enemy.Start Weapon Trace`
  (`/Game/Blueprints/BPC_AttackSystem.StartSwordTrace` (`self.BPC_AttackSystem`)))

(event `/Game/Blueprints/Enemies/BPI_Enemy.End Weapon Trace`
  (`/Game/Blueprints/BPC_AttackSystem.StopSwordTrace` (`self.BPC_AttackSystem`)))

(fn `GetWeaponTrace`
  (returns (Top :type "Vector Structure") (Bottom :type "Vector Structure"))
  (bind _weapon_combat (`self.Weapon_Combat`))
  (return (`SceneComponent.GetSocketLocation` _weapon_combat "Top") (`SceneComponent.GetSocketLocation` _weapon_combat "Bottom")))

(fn `Set Weapon Visibility`
  (params (Target :type "SceneComponent Object Reference") (NewHidden :type Boolean))
  (`SceneComponent.SetHiddenInGame` Target NewHidden false))

(fn `UserConstructionScript`
  (`parent.UserConstructionScript`))