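; Melee enemy Claire, a child enemy Blueprint that carries a teddy as her idle weapon mesh and drops a teddy item on death.
; BeginPlay sets that mesh and creates a dynamic dissolve material with a glowing pink color.
; After the parent death logic, a one-shot sequence plays her death sound, swaps the weapon mesh to Stern, spawns BP_Item_Teddy and runs a timeline driving the body's dissolve.
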(event `self.ReceiveBeginPlay`
  (`parent.ReceiveBeginPlay`)
  (`StaticMeshComponent.SetStaticMesh` (`self.Weapon_Idle`) "/Game/Art/EnemySmall/Waffen/Teddy/TeddyMesh.TeddyMesh")
  (bind _returnvalue (`PrimitiveComponent.CreateDynamicMaterialInstance` (`self.Mesh`) 0 "/Game/Art/EnemySmall/M_Dissolve_Inst.M_Dissolve_Inst" "None"))
  (bind _output_get (set `self.ClaireDed` _returnvalue))
  (`MaterialInstanceDynamic.SetVectorParameterValue` _output_get "DissolveColor" (struct :`R` 100.0 :`G` 7.239014 :`B` 45.194393 :`A` 1.0)))

(event `/Game/Blueprints/Enemies/BP_Enemy_Parent.Death Parent`
  (bind (_returnvalue_location _returnvalue_rotation) (`KismetMathLibrary.BreakTransform` (`self.GetTransform`)))
  (bind _claireded (`self.ClaireDed`))
  (`parent.Death Parent`)
  (`/Engine/EditorBlueprintResources/StandardMacros.DoOnce` false
    (:`Completed`
      ;[1 1 1] done
      (`FMODBlueprintStatics.PlayEvent2D` "/Game/FMOD/Events/ClaireDeath.ClaireDeath")
      (`StaticMeshComponent.SetStaticMesh` (`self.Weapon_Idle`) "/Game/Art/Particle/DashCooldow/Stern.Stern")
      (`|SpawnActorFromClass` "/Game/Blueprints/Interactables/BP_Item_Teddy.BP_Item_Teddy_C" (`KismetMathLibrary.MakeTransform` _returnvalue_location _returnvalue_rotation) "Undefined" "MultiplyWithRoot" null null)
      (bind (_direction _dissolve _smoothnes) (`Timeline|Timeline`)
        (:`Update`
          (`MaterialInstanceDynamic.SetScalarParameterValue` _claireded "Dissolve" _dissolve)
          (`MaterialInstanceDynamic.SetScalarParameterValue` _claireded "TransitionSmoothness" _smoothnes))))))

(fn `UserConstructionScript`
  (`parent.UserConstructionScript`))