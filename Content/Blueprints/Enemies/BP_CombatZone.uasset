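; BP_CombatZone is an enemy combat zone that tells its assigned enemies when the player enters or leaves.
; CombatArea overlaps send enter and player-exit messages to every valid enemy in EnemiesInZone, and an exit message to any enemy leaving the area.
; The construction script scales CombatArea and SpawnArea from outer and inner sphere scaling variables; SpawnArea's overlap event does nothing.
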(event `self.CombatArea.OnComponentBeginOverlap`
  (params (OverlappedComponent :type "PrimitiveComponent Object Reference") (OtherActor :type "Actor Object Reference") (OtherComp :type "PrimitiveComponent Object Reference") (OtherBodyIndex :type Integer) (bFromSweep :type Boolean) (SweepResult :type "HitResult Structure (by ref)"))
  (if (`self.ActorHasTag` OtherActor "Player")
    (for _array_element (`self.Enemies in Zone`)
      (`/Engine/EditorBlueprintResources/StandardMacros.IsValid` _array_element
        (:`Is Valid`
          (message `/Game/Blueprints/Enemies/BPI_Enemy.EnterCombatZone` _array_element))))))

(event `self.CombatArea.OnComponentEndOverlap`
  (params (OverlappedComponent :type "PrimitiveComponent Object Reference") (OtherActor :type "Actor Object Reference") (OtherComp :type "PrimitiveComponent Object Reference") (OtherBodyIndex :type Integer))
  (if (`self.ActorHasTag` OtherActor "Enemy")
    (`/Engine/EditorBlueprintResources/StandardMacros.IsValid` OtherActor
      (:`Is Valid`
        (message `/Game/Blueprints/Enemies/BPI_Enemy.ExitCombatZone` OtherActor)))
    (elif (`self.ActorHasTag` OtherActor "Player")
      (for _array_element (`self.Enemies in Zone`)
        (`/Engine/EditorBlueprintResources/StandardMacros.IsValid` _array_element
          (:`Is Valid`
            (message `/Game/Blueprints/Enemies/BPI_Enemy.Player Exit Combatzone` _array_element)))))))

(event `self.SpawnArea.OnComponentBeginOverlap`
  (params (OverlappedComponent :type "PrimitiveComponent Object Reference") (OtherActor :type "Actor Object Reference") (OtherComp :type "PrimitiveComponent Object Reference") (OtherBodyIndex :type Integer) (bFromSweep :type Boolean) (SweepResult :type "HitResult Structure (by ref)")))

(fn `UserConstructionScript`
  (`SceneComponent.SetWorldScale3D` (`self.CombatArea`) (* (1.0 1.0 1.0) (`self.Outer Sphere Scaling`)))
  (`SceneComponent.SetWorldScale3D` (`self.SpawnArea`) (* (1.0 1.0 1.0) (`self.Inner Sphere Scaling`))))