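; Health component for enemies that tracks maximum and current HP.
; On BeginPlay it fills both values from the owner's GetStatsMessage call.
; TakeDMG records the damage received, subtracts it from current HP and returns whether HP has reached zero or below, leaving any death response to the caller.
; If HP is already depleted, it returns true without subtracting again.
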(event `self.ReceiveBeginPlay`
  (bind _max_hp (message `/Game/Blueprints/Enemies/BPI_Damagable.Get Stats` (`self.GetOwner`)))
  (bind _output_get (set `self.Max HP` _max_hp))
  (set `self.Current HP` _output_get))

(fn `Take DMG`
  (params (`DMG Dealt` :type "Float (double-precision)"))
  (returns (Dead :type Boolean))
  (set `self.DMG Received` `DMG Dealt`)
  (if (<= (`self.Current HP`) 0.0)
    (return true)
    (else
      (set `self.Current HP` (- (`self.Current HP`) (`self.DMG Received`)))
      (if (<= (`self.Current HP`) 0.0)
        (return true)
        (else
          (return false))))))