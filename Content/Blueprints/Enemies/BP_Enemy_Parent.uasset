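; Base enemy Blueprint that switches between Idle, Combat and Retreat as the player and enemy cross combat zone boundaries.
; Zone events write state and player target to the Blackboard.
; Leaving the zone during combat triggers retreat to the stored spawn transform, then Combat or Idle depending on player presence.
; Damage goes through a health component that decides actor destruction, while getters expose max health, spawn transform and an empty GetBT.
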(event `self.ReceiveBeginPlay`
  (set `self.Spawn Transform` (`self.GetTransform`)))

(event `/Game/Blueprints/Enemies/BPI_Enemy.EnterCombatZone`
  ;[1 1 1] Player entered Combat Zone
  (set `self.Player in Zone` true)
  (switch `/Game/Blueprints/Enemies/AI/E_Enemy_AIStates` (`self.AIStates`)
    (:`NewEnumerator0`
      (`self.Set AI State` "NewEnumerator1")
      (`self.Set AI PlayerCharacter` (`GameplayStatics.GetPlayerCharacter` 0)))))

(event `/Game/Blueprints/Enemies/BPI_Enemy.Player Exit Combatzone`
  ;[1 1 1] Player left Combat Zone
  (set `self.Player in Zone` false))

(event `/Game/Blueprints/Enemies/BPI_Enemy.ExitCombatZone`
  ;[1 1 1] Enemy left Combat Zone
  (switch `/Game/Blueprints/Enemies/AI/E_Enemy_AIStates` (`self.AIStates`)
    (:`NewEnumerator1`
      (`self.Set AI State` "NewEnumerator2")
      (`self.Set AI PlayerCharacter` null))))

(event `/Game/Blueprints/Enemies/BPI_Enemy.BackOnSpawnTransform`
  ;[1 1 1] Enemy retreated successfully
  (switch `/Game/Blueprints/Enemies/AI/E_Enemy_AIStates` (`self.AIStates`)
    (:`NewEnumerator2`
      (if (`self.Player in Zone`)
        (`self.Set AI State` "NewEnumerator1")
        (`self.Set AI PlayerCharacter` (`GameplayStatics.GetPlayerCharacter` 0))
        (else
          (`self.Set AI State` "NewEnumerator0")
          (`self.Set AI PlayerCharacter` null))))))

(event `/Game/Blueprints/Enemies/BPI_Damagable.Take DMG`
  (params (`DMG amount` :type "Float (double-precision)"))
  (bind _bpc_healthsystem (`self.BPC_Healthsystem`))
  (bind _dead (`/Game/Blueprints/Enemies/BPC_Healthsystem.Take DMG` _bpc_healthsystem `DMG amount`))
  (`KismetSystemLibrary.PrintString` (`KismetStringLibrary.Conv_DoubleToString` (`/Game/Blueprints/Enemies/BPC_Healthsystem.Current HP` _bpc_healthsystem)))
  (if _dead
    (`self.K2_DestroyActor`)))

(fn `Get Stats`
  (returns (`Max HP` :type "Float (double-precision)"))
  (return (`/Game/Blueprints/Enemies/PDA_Enemy_Parent.Max Health` (`self.Enemy Stats`))))

(fn `GetBT`
  (returns (BT :type "BehaviorTree Object Reference"))
  (return null))

(fn `GetSpawnTransform`
  (returns (SpawnTransform :type "Transform Structure"))
  (return (`self.Spawn Transform`)))

(fn `UserConstructionScript`)