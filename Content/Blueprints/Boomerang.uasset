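; Boomerang Blueprint, apparently an early draft of a homing projectile; no movement or hit logic runs in its graphs.
; BeginPlay fires a debug-drawn visibility sphere trace, with identical start and end built from the forward vector alone, ignoring actor location and discarding the result.
; FindPlayerCharacter selects a "Player"-tagged third-person character by shortest distance as HomingTarget and returns its SceneComponent, but nothing here calls it.
; The Rotation_T node is unconnected.
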(event `self.ReceiveBeginPlay`
  (bind _returnvalue (`self.GetActorForwardVector`))
  (bind _returnvalue_2 (+ _returnvalue (* _returnvalue 2000.0)))
  (`KismetSystemLibrary.SphereTraceSingle` :`Start` _returnvalue_2 :`End` _returnvalue_2 :`Radius` 15.0 :`TraceChannel` "TraceTypeQuery1" :`DrawDebugType` "ForDuration"))

(fn `FindPlayerCharacter`
  (returns (HomingTarget :type "SceneComponent Object Reference"))
  (bind _outactors (`GameplayStatics.GetAllActorsOfClassWithTag` "/Game/ThirdPerson/Blueprints/BP_ThirdPersonCharacter.BP_ThirdPersonCharacter_C" "Player"))
  (for _array_element _outactors
    (bind _returnvalue (`KismetMathLibrary.VSize` (- (`self.K2_GetActorLocation` _array_element) (`self.K2_GetActorLocation`))))
    (if (< _returnvalue (`self.Distance`))
      (set `self.Distance` _returnvalue)
      (set `self.HomingTarget` _array_element)))
  (return (`self.GetComponentByClass` (`self.HomingTarget`) "/Script/Engine.SceneComponent")))

(fn `UserConstructionScript`)