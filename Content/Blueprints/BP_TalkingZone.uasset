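; BP_TalkingZone is a one-shot trigger box that shows dialogue text with sound when the player enters it.
; The first overlap by a "Player"-tagged actor sets the global audio parameter "Dialog", plays the KIMSOUND 2D event and displays a WB_TalkingZone widget with the Text variable.
; A timer of TimeTillDestroy then removes the widget and resets the parameter.
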(event `CreateWidget`
  (bind _returnvalue (`|CreateWidget` "/Game/UI/WB_TalkingZone.WB_TalkingZone_C" (`GameplayStatics.GetPlayerController` 0)))
  (bind _output_get (set `self.TalkingZone` _returnvalue))
  (`UserWidget.AddToViewport` _output_get 0))

(event `self.Box.OnComponentBeginOverlap`
  (params (OverlappedComponent :type "PrimitiveComponent Object Reference") (OtherActor :type "Actor Object Reference") (OtherComp :type "PrimitiveComponent Object Reference") (OtherBodyIndex :type Integer) (bFromSweep :type Boolean) (SweepResult :type "HitResult Structure (by ref)"))
  (if (`self.ActorHasTag` OtherActor "Player")
    (`/Engine/EditorBlueprintResources/StandardMacros.DoOnce` false
      (:`Completed`
        (`FMODBlueprintStatics.SetGlobalParameterByName` "Dialog" 1.0)
        (`FMODBlueprintStatics.PlayEvent2D` (`self.KIMSOUND`))
        (`self.CreateWidget`)
        (`/Game/UI/WB_TalkingZone.SetText` (`self.TalkingZone`) (`self.Text`))
        (`KismetSystemLibrary.K2_SetTimerDelegate` (delegate `RemoveWidget`) (`self.TimeTillDestroy`))))))

(event `RemoveWidget`
  (`Widget.RemoveFromParent` (`self.TalkingZone`))
  (`FMODBlueprintStatics.SetGlobalParameterByName` "Dialog"))

(fn `UserConstructionScript`)