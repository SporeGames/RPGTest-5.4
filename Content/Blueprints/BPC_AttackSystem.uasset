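; Actor component that gives BP_ThirdPersonCharacter a four-step sword and kick melee combo with hit detection.
; Attack input starts montages by AttackIndex, buffering presses mid-attack for SwordAttackCombo to continue or reset the chain.
; Sword hits use a timer-looped sphere trace between blade points with a DoOnce cooldown, while SphereTrace checks stabs and kicks once.
; Hits on "Damagable"-tagged actors apply damage, camera shake and blood particles.
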(event `self.ReceiveBeginPlay`
  (bind _asbp_third_person_character (cast `/Game/ThirdPerson/Blueprints/BP_ThirdPersonCharacter` (`self.GetOwner`)))
  (bind _output_get (set `self.CharacterBP` _asbp_third_person_character))
  (set `self.Mesh` (`Character.Mesh` _output_get)))

(event `EnhancedInput|/Game/ThirdPerson/Input/Actions/IA_Attack`
  (params (ActionValue :type Boolean) (ElapsedSeconds :type "Float (double-precision)") (TriggeredSeconds :type "Float (double-precision)") (InputAction :type "InputAction Object Reference" :default "/Game/ThirdPerson/Input/Actions/IA_Attack.IA_Attack"))
  ;[1 1 1] ComboSystem
  ;;[1 1 1] Attack Input
  (:`Started`
    (if (`self.canAttack`)
      (`self.SwordAttack`))))

(event `Attack1`
  ;[1 1 1] ComboSystem
  ;;[1 1 1] Attack 1
  (`/Engine/EditorBlueprintResources/StandardMacros.DoOnce` false :!label _label
    (:`Completed`
      (`KismetSystemLibrary.Delay` 0.1)
      (`|PlayMontage` (`self.Mesh`) "/Game/Characters/RPG_Character/Animations/SwordAttacks/Attack1_Montage.Attack1_Montage"
        (:`then`
          (set `self.attackIndex` 1)
          (goto _label :!via `Reset`))))))

(event `SwordAttack`
  ;[1 1 1] ComboSystem
  ;;[1 1 1] Sword Attack
  (if (`self.isAttacking`)
    (set `self.saveAttack` true)
    (else
      (set `self.isAttacking` true)
      (switch `int` (`self.attackIndex`) :!label _label_2
        (:`0`
          (`self.Attack1`))
        (:`1`
          (`self.Attack2`))
        (:`2`
          (`self.Attack 3`))
        (:`3`
          (`self.Attack 4`))))))

(event `Attack2`
  ;[1 1 1] ComboSystem
  ;;[1 1 1] Attack 2
  (`/Engine/EditorBlueprintResources/StandardMacros.DoOnce` false :!label _label_3
    (:`Completed`
      (`KismetSystemLibrary.Delay` 0.1)
      (`|PlayMontage` (`self.Mesh`) "/Game/Characters/RPG_Character/Animations/SwordAttacks/Attack2_Montage.Attack2_Montage"
        (:`then`
          (set `self.attackIndex` 2)
          (goto _label_3 :!via `Reset`))))))

(event `SwordAttackCombo`
  ;[1 1 1] ComboSystem
  ;;[1 1 1] Combo Continue
  (if (`self.saveAttack`)
    (set `self.saveAttack` false)
    (goto _label_2)
    (else
      (`self.StopCombo`))))

(event `Attack 3`
  ;[1 1 1] ComboSystem
  ;;[1 1 1] Attack 3
  (`/Engine/EditorBlueprintResources/StandardMacros.DoOnce` false :!label _label_4
    (:`Completed`
      (`KismetSystemLibrary.Delay` 0.1)
      (`|PlayMontage` (`self.Mesh`) "/Game/Characters/RPG_Character/Animations/SwordAttacks/Kick_Montage.Kick_Montage"
        (:`then`
          (set `self.attackIndex` 3)
          (goto _label_4 :!via `Reset`))))))

(event `StopCombo`
  ;[1 1 1] ComboSystem
  ;;[1 1 1] Stop Combo / Attack
  (set `self.isAttacking` false)
  (set `self.attackIndex` 0))

(event `Attack 4`
  ;[1 1 1] ComboSystem
  ;;[1 1 1] Attack 4
  (`/Engine/EditorBlueprintResources/StandardMacros.DoOnce` false :!label _label_5
    (:`Completed`
      (`KismetSystemLibrary.Delay` 0.1)
      (`|PlayMontage` (`self.Mesh`) "/Game/Characters/RPG_Character/Animations/SwordAttacks/Attack3_Montage.Attack3_Montage"
        (:`then`
          (set `self.attackIndex` 4)
          (goto _label_5 :!via `Reset`))))))

(event `StartSwordTrace`
  ;[1 1 1] SwordTrace
  (bind _returnvalue (`KismetSystemLibrary.K2_SetTimerDelegate` (delegate `SwordTraceLoop`) 0.001 true))
  (set `self.SwordTraceLoopp` _returnvalue))

(event `SphereTrace`
  (bind _returnvalue (`SceneComponent.K2_GetComponentLocation` (`/Game/ThirdPerson/Blueprints/BP_ThirdPersonCharacter.SphereTrace` (`self.CharacterBP`))))
  ;[1 1 1] Sphere Trace for Stab and Kick
  (bind (_outhit _returnvalue_2) (`KismetSystemLibrary.SphereTraceSingle` _returnvalue _returnvalue 50.0 "TraceTypeQuery1"))
  (if _returnvalue_2
    (bind (_bblockinghit _binitialoverlap _time _distance _location _impactpoint _normal _impactnormal _physmat _hitactor) (`GameplayStatics.BreakHitResult` _outhit))
    (if (`Actor.ActorHasTag` _hitactor "Damagable")
      (`GameplayStatics.ApplyDamage` _hitactor 10.0)
      (`GameplayStatics.PlayWorldCameraShake` "/Game/Blueprints/BP_SwordHitCameraShack.BP_SwordHitCameraShack_C" _location 0.0 2000.0)
      (`GameplayStatics.SpawnEmitterAtLocation` "/Game/Realistic_Starter_VFX_Pack_Vol2/Particles/Blood/P_Blood_Splat_Cone.P_Blood_Splat_Cone" _location (`KismetMathLibrary.MakeRotFromXY` _normal _normal) (0.4 0.4 0.4)))))

(event `SwordTraceLoop`
  ;[1 1 1] SwordTrace
  (bind (_outhit _returnvalue) (`KismetSystemLibrary.SphereTraceSingle` (`SceneComponent.K2_GetComponentLocation` (`/Game/ThirdPerson/Blueprints/BP_ThirdPersonCharacter.SwordTopPoint` (`self.CharacterBP`))) (`SceneComponent.K2_GetComponentLocation` (`/Game/ThirdPerson/Blueprints/BP_ThirdPersonCharacter.SwordBottemPoint` (`self.CharacterBP`))) 25.0 "TraceTypeQuery1"))
  (if _returnvalue
    (bind (_bblockinghit _binitialoverlap _time _distance _location _impactpoint _normal _impactnormal _physmat _hitactor) (`GameplayStatics.BreakHitResult` _outhit))
    (if (`Actor.ActorHasTag` _hitactor "Damagable")
      (`/Engine/EditorBlueprintResources/StandardMacros.DoOnce` false :!label _label_6
        (:`Completed`
          (`GameplayStatics.ApplyDamage` _hitactor 10.0)
          (`GameplayStatics.PlayWorldCameraShake` "/Game/Blueprints/BP_SwordHitCameraShack.BP_SwordHitCameraShack_C" _location 0.0 2000.0)
          (`GameplayStatics.SpawnEmitterAtLocation` "/Game/Realistic_Starter_VFX_Pack_Vol2/Particles/Blood/P_Blood_Splat_Cone.P_Blood_Splat_Cone" _location (`KismetMathLibrary.MakeRotFromXY` _normal _normal) (0.4 0.4 0.4))
          (`KismetSystemLibrary.Delay` 0.5)
          (goto _label_6 :!via `Reset`))))))

(event `StopSwordTrace`
  ;[1 1 1] SwordTrace
  (`KismetSystemLibrary.K2_ClearAndInvalidateTimerHandle` (`self.SwordTraceLoopp`)))