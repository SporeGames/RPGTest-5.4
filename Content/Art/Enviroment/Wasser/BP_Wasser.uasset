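; BP_Wasser is a water actor that spawns player splash Niagara effects.
; BeginPlay caches the third-person character, and Tick flags it as moving when its velocity is non-zero.
; When a "Player"-tagged actor enters the box while moving, a looping timer repeatedly spawns splashes at the character's XY and a fixed height.
; The overlap also prints the speed for debugging, and nothing here stops the timer.
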(event `CustomEvent`
  (bind (_returnvalue_x _returnvalue_y) (`KismetMathLibrary.BreakVector` (`self.K2_GetActorLocation` (`self.As BP Third Person Character`))))
  (`NiagaraFunctionLibrary.SpawnSystemAtLocation` "/Game/Art/Enviroment/Wasser/NS_WasserSpritzerPlayer.NS_WasserSpritzerPlayer" (`KismetMathLibrary.MakeVector` _returnvalue_x _returnvalue_y -10.0)))

(event `self.ReceiveTick`
  (params (DeltaSeconds :type "Float (single-precision)"))
  (bind _output_get (set `self.Moving?` (> (`KismetMathLibrary.VSize` (`MovementComponent.Velocity` (`Character.CharacterMovement` (`self.As BP Third Person Character`)))) 0.0))))

(event `self.ReceiveBeginPlay`
  (bind _asbp_third_person_character (cast `/Game/ThirdPerson/Blueprints/BP_ThirdPersonCharacter` (`GameplayStatics.GetPlayerPawn` 0)))
  (set `self.As BP Third Person Character` _asbp_third_person_character))

(event `self.ReceiveActorBeginOverlap`
  (params (OtherActor :type "Actor Object Reference")))

(event `self.Box.OnComponentBeginOverlap`
  (params (OverlappedComponent :type "PrimitiveComponent Object Reference") (OtherActor :type "Actor Object Reference") (OtherComp :type "PrimitiveComponent Object Reference") (OtherBodyIndex :type Integer) (bFromSweep :type Boolean) (SweepResult :type "HitResult Structure (by ref)"))
  (if (`self.ActorHasTag` OtherActor "Player")
    (`KismetSystemLibrary.PrintString` (`KismetStringLibrary.Conv_DoubleToString` (`KismetMathLibrary.VSize` (`MovementComponent.Velocity` (`Character.CharacterMovement` (`self.As BP Third Person Character`))))))
    (if (`self.Moving?`)
      (`KismetSystemLibrary.K2_SetTimerDelegate` (delegate `CustomEvent`) 0.05 true true))))

(fn `UserConstructionScript`)