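; Game instance that owns the BP_SaveGame object, loading it synchronously on Init or creating and saving one if the slot is empty.
; SavePlayer, SaveSound and SaveMouse update their part of the save and write it to the slot, with async optional for player data.
; GetSavedGameData exposes the save object, and OnGameLoaded is called only when an async load completes.
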(event `self.ReceiveInit`
  (`self.LoadGameData` false))

(event `/Game/Save_Load/BPI_SaveGame.SaveGameData`
  (params (Async :type Boolean))
  (if Async
    (`AsyncActionHandleSaveGame.AsyncSaveGameToSlot` (`self.SaveGame`) (`self.Slot_Name`))
    (else
      (`GameplayStatics.SaveGameToSlot` (`self.SaveGame`) (`self.Slot_Name`)))))

(event `/Game/Save_Load/BPI_SaveGame.LoadGameData`
  (params (Async :type Boolean))
  (bind _returnvalue (`GameplayStatics.DoesSaveGameExist` (`self.Slot_Name`)))
  (if _returnvalue
    (if Async
      ;[1 1 1] Async loads in background
      (bind _savegame (`AsyncActionHandleSaveGame.AsyncLoadGameFromSlot` (`self.Slot_Name`))
        (:`Completed`
          (bind _asbp_save_game (cast `/Game/Save_Load/BP_SaveGame` _savegame))
          (set `self.SaveGame` _asbp_save_game)
          (`self.OnGameLoaded`)))
      (else
        (bind _returnvalue_2 (`GameplayStatics.LoadGameFromSlot` (`self.Slot_Name`)))
        (bind _asbp_save_game_2 (cast `/Game/Save_Load/BP_SaveGame` _returnvalue_2))
        (set `self.SaveGame` _asbp_save_game_2)))
    (else
      (bind _returnvalue_3 (`GameplayStatics.CreateSaveGameObject` "/Game/Save_Load/BP_SaveGame.BP_SaveGame_C"))
      (bind _output_get (set `self.SaveGame` _returnvalue_3))
      (`GameplayStatics.SaveGameToSlot` _output_get (`self.Slot_Name`)))))

(event `/Game/Save_Load/BPI_SaveGame.SavePlayer`
  (params (`Player Save` :type "/Game/Save_Load/S_Player_SaveGame Structure") (Async :type Boolean))
  (set `/Game/Save_Load/BP_SaveGame.Player Save` `Player Save` (`self.SaveGame`))
  (`self.SaveGameData` Async))

(event `/Game/Save_Load/BPI_SaveGame.SaveSound`
  (params (Sound :type "/Game/Save_Load/S_Sound_SaveGame Structure"))
  (set `/Game/Save_Load/BP_SaveGame.SOundSave` Sound (`self.SaveGame`))
  (`self.SaveGameData` false))

(event `/Game/Save_Load/BPI_SaveGame.SaveMouse`
  (params (Mouse :type "/Game/Save_Load/S_Mouse_SaveGame Structure"))
  (set `/Game/Save_Load/BP_SaveGame.MouseSave` Mouse (`self.SaveGame`))
  (`self.SaveGameData` false))

(fn `GetSavedGameData`
  (returns (SaveGame :type "/Game/Save_Load/BP_SaveGame Object Reference"))
  (return (`self.SaveGame`)))